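; BP_Ladder is a ladder actor that marks itself as climbable to characters standing at either of its entrances.
; The construction script stacks LadderMesh segments to fit LadderHeight, adds query-collision steps at StepHeight intervals, and stores the first and last step.
; It also sizes and places entrance boxes at the bottom and top.
; Overlapping either box toggles PotentialLadder on the BaseCharacter_BP's UMC component.
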(event OnComponentBeginOverlap(Entrance_1)
  (params (OverlappedComponent :type Primitive%20Component%20Object%20Reference) (OtherActor :type Actor%20Object%20Reference) (OtherComp :type Primitive%20Component%20Object%20Reference) (OtherBodyIndex :type Integer) (bFromSweep :type Boolean) (SweepResult :type Hit%20Result%20Structure%20%28by%20ref%29))
  (CallFunction|UpdateLadderonChar OtherActor true))

(event OnComponentEndOverlap(Entrance_1)
  (params (OverlappedComponent :type Primitive%20Component%20Object%20Reference) (OtherActor :type Actor%20Object%20Reference) (OtherComp :type Primitive%20Component%20Object%20Reference) (OtherBodyIndex :type Integer))
  (CallFunction|UpdateLadderonChar OtherActor false))

(event OnComponentBeginOverlap(Entrance_2)
  (params (OverlappedComponent :type Primitive%20Component%20Object%20Reference) (OtherActor :type Actor%20Object%20Reference) (OtherComp :type Primitive%20Component%20Object%20Reference) (OtherBodyIndex :type Integer) (bFromSweep :type Boolean) (SweepResult :type Hit%20Result%20Structure%20%28by%20ref%29))
  (CallFunction|UpdateLadderonChar OtherActor true))

(event OnComponentEndOverlap(Entrance_2)
  (params (OverlappedComponent :type Primitive%20Component%20Object%20Reference) (OtherActor :type Actor%20Object%20Reference) (OtherComp :type Primitive%20Component%20Object%20Reference) (OtherBodyIndex :type Integer))
  (CallFunction|UpdateLadderonChar OtherActor false))

(event EventBeginPlay)

(event Collision|EventActorBeginOverlap
  (params (OtherActor :type Actor%20Object%20Reference)))

(event EventTick
  (params (DeltaSeconds :type Float%20%28single-precision%29)))

(fn ConstructionScript
  (CallFunction|InitializeLadderMesh)
  (CallFunction|InitializeLadderSteps)
  (CallFunction|InitializeEnterances))

(fn InitializeLadderMesh
  (bind _returnvalue (Transformation|GetActorLocation))
  (bind (_x _y _z) (Math|Vector|BreakVector _returnvalue))
  (Utilities|IsValid (Variables|UMC|GetLadderMesh)
    (:Is%20Valid
      (LocalVariables|SetTempHeightMesh (.Z (Math|Vector|BreakVector (.Max (Utilities|Struct|BreakBox (StaticMesh|GetBoundingBox (Variables|UMC|GetLadderMesh)))))))
      (for _index (range 0 (- (Math|Float|Truncate (/ (Variables|UMC|GetLadderHeight) (LocalVariables|GetTempHeightMesh))) 1))
        (bind _returnvalue_2 (AddComponent|AddStaticMeshComponent false))
        (bind _output_get (LocalVariables|SetTempMesh _returnvalue_2))
        (Components|StaticMesh|SetStaticMesh _output_get (Variables|UMC|GetLadderMesh))
        (Transformation|SetWorldLocation (LocalVariables|GetTempMesh) (Math|Vector|MakeVector _x _y (+ _z (* _index (LocalVariables|GetTempHeightMesh)))) false false)
        (Collision|SetCollisionEnabled (LocalVariables|GetTempMesh) "PhysicsOnly"))
      (Collision|SetCollisionEnabled (LocalVariables|GetTempMesh) "NoCollision"))))

(fn InitializeEnterances
  (bind _returnvalue (Transformation|GetActorLocation))
  (bind _entrance_1 (Variables|Default|GetEntrance_1))
  (bind _entrance_2 (Variables|Default|GetEntrance_2))
  (bind _laddermesh (Variables|UMC|GetLadderMesh))
  (bind _returnvalue_2 (StaticMesh|GetBoundingBox _laddermesh))
  (bind (_x _y _z) (Math|Vector|BreakVector _returnvalue))
  (bind _max (Utilities|Struct|BreakBox _returnvalue_2))
  (bind _z_2 (Math|Vector|BreakVector _max))
  (Utilities|IsValid (Variables|UMC|GetLadderMesh)
    (:Is%20Valid
      (Utilities|FlowControl|Sequence
        (:then_0
          (Components|Box|SetBoxExtent _entrance_1 (Variables|UMC|GetEntrance_1_Size) true)
          (Transformation|SetWorldLocation _entrance_1 (+ (Transformation|GetActorLocation) (Variables|UMC|GetEntrance_1_Offset)) false false))
        (:then_1
          (Components|Box|SetBoxExtent _entrance_2 (Variables|UMC|GetEntrance_2_Size) true)
          (Transformation|SetWorldLocation _entrance_2 (+ (Math|Vector|MakeVector _x _y (+ _z (* (Math|Float|Truncate (/ (Variables|UMC|GetLadderHeight) _z_2)) _z_2))) (Variables|UMC|GetEntrance_2_Offset)) false false))))))

(fn InitializeLadderSteps
  (bind _returnvalue (Transformation|GetActorLocation))
  (bind _returnvalue_2 (Transformation|GetActorLocation))
  (bind (_x _y _z) (Math|Vector|BreakVector _returnvalue_2))
  (bind (_x_2 _y_2 _z_2) (Math|Vector|BreakVector _returnvalue))
  (Utilities|IsValid (Variables|UMC|GetStepMesh)
    (:Is%20Valid
      ;[1 1 1] Intialize & store first step
      (bind _returnvalue_3 (AddComponent|AddStaticMeshComponent false))
      (bind _output_get (Variables|Default|SetFirstStep _returnvalue_3))
      (Components|StaticMesh|SetStaticMesh _output_get (Variables|UMC|GetLadderMesh))
      (Transformation|SetWorldLocation (Variables|Default|GetFirstStep) (Math|Vector|MakeVector _x_2 _y_2 (+ _z_2 (Variables|UMC|GetStepHeight))) false false)
      (Collision|SetCollisionEnabled (Variables|Default|GetFirstStep) "QueryOnly")
      (for _index (range 2 (Math|Float|Truncate (/ (Variables|UMC|GetLadderHeight) (Variables|UMC|GetStepHeight))))
        (bind _returnvalue_4 (AddComponent|AddStaticMeshComponent false))
        (Utilities|FlowControl|Sequence
          (:then_0
            (Components|StaticMesh|SetStaticMesh _returnvalue_4 (Variables|UMC|GetStepMesh)))
          (:then_1
            (Transformation|SetWorldLocation _returnvalue_4 (Math|Vector|MakeVector _x _y (+ _z (* _index (Variables|UMC|GetStepHeight)))) false false))
          (:then_2
            (Collision|SetCollisionEnabled _returnvalue_4 "QueryOnly"))
          (:then_3
            (LocalVariables|SetTempStepMesh _returnvalue_4))))
      (Variables|Default|SetLastStep (LocalVariables|GetTempStepMesh)))))

(fn UpdateLadderonChar
  (params (InActor :type Actor%20Object%20Reference) (bInEnable :type Boolean))
  (bind _asbase_character_bp (Utilities|Casting|CastToBaseCharacter_BP InActor))
  (Utilities|IsValid (Variables|/Game/UltimateCharacter/Blueprints/Characters/BaseCharacter_BP.BaseCharacter_BP_C|GetUMC _asbase_character_bp)
    (:Is%20Valid
      (Variables|/Game/UltimateCharacter/Blueprints/Components/UMC.UMC_C|SetbPotentialLadder (Variables|/Game/UltimateCharacter/Blueprints/Characters/BaseCharacter_BP.BaseCharacter_BP_C|GetUMC _asbase_character_bp) bInEnable))))