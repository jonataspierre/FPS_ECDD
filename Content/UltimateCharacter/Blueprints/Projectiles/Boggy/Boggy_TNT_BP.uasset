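; Boggy_TNT_BP is a TNT projectile with a spark particle snapped to the mesh's "Sparks" socket on BeginPlay.
; When projectile movement stops, it stores the hit result.
; On the authority, if not yet exploded, it logs the hit actor, turns on mesh physics simulation and makes the mesh ignore the Camera channel.
; The explosion itself is not handled in this graph.
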(event OnProjectileStop(ProjectileMovement)
  (params (ImpactResult :type Hit%20Result%20Structure%20%28by%20ref%29))
  (bind _mesh (Variables|Character|GetMesh))
  (Variables|Default|SetHitResult ImpactResult)
  (if (and (Utilities|Enum|Equal(Enum) (Networking|GetLocalRole) "ROLE_Authority") (not (Variables|Default|GetbExploded)))
    (CallFunction|ShowDebugMessage "BaseProjectile_BP" "OnStopProjectile" (Utilities|String|Append (Utilities|GetDisplayName self) " stopped by " (Utilities|GetDisplayName (.HitActor (Collision|BreakHitResult (Variables|Default|GetHitResult))))) "NewEnumerator0")
    ;[1 1 1] Set simulate physics
    (Physics|SetSimulatePhysics _mesh true)
    (Collision|SetCollisionResponsetoChannel _mesh "ECC_Camera" "ECR_Ignore")))

(event EventBeginPlay
  (|CallParentFunction)
  (Transformation|AttachComponentToComponent (Variables|Default|GetParticle) (Variables|Character|GetMesh) "Sparks" "SnapToTarget" "SnapToTarget" "SnapToTarget" true))

(event Collision|EventActorBeginOverlap
  (params (OtherActor :type Actor%20Object%20Reference))
  (|CallParentFunction OtherActor) ; This node is disabled and will not be called.\nDrag off pins to build functionality.
)

(event EventTick
  (params (DeltaSeconds :type Float%20%28single-precision%29))
  (|CallParentFunction DeltaSeconds) ; This node is disabled and will not be called.\nDrag off pins to build functionality.
)

(fn ConstructionScript
  (|CallParentFunction))