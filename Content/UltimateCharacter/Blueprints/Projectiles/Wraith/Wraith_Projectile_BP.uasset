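; Wraith projectile Blueprint that halts when it nears a surface below it and drifts slightly upward ahead of its explosion.
; After the parent Tick, it runs a short downward Visibility line trace, drawn when ShowDebug is set.
; The first hit, gated by DoOnce, stops ProjectileMovement and sets a slightly negative gravity scale to create the lift.
; The explosion itself is not implemented in this graph.
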(event EventBeginPlay
  (|CallParentFunction) ; This node is disabled and will not be called.\nDrag off pins to build functionality.
)

(event Collision|EventActorBeginOverlap
  (params (OtherActor :type Actor%20Object%20Reference))
  (|CallParentFunction OtherActor) ; This node is disabled and will not be called.\nDrag off pins to build functionality.
)

(event EventTick
  (params (DeltaSeconds :type Float%20%28single-precision%29))
  (bind _returnvalue (Transformation|GetActorLocation))
  (bind _projectilemovement (Variables|Default|GetProjectileMovement))
  (|CallParentFunction DeltaSeconds)
  (bind _returnvalue_2 (Collision|LineTraceByChannel _returnvalue (+ _returnvalue "0, 0,-30.000000") "TraceTypeQuery1" false 0 (select (Variables|Default|GetbShowDebug) "ForDuration" "None")))
  (if _returnvalue_2
    ;[1 1 1] Stop projectile movement and send a little bit up before explosion
    (Utilities|FlowControl|DoOnce false
      (:Completed
        (Components|Movement|StopMovementImmediately _projectilemovement)
        (Variables|/Script/Engine.ProjectileMovementComponent|SetProjectileGravityScale _projectilemovement -0.01)))))

(fn ConstructionScript
  (|CallParentFunction))