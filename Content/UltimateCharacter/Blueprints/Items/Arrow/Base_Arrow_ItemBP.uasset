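; Base arrow item that characters pick up as bow ammo, tagged from its arrow class's projectile config and never respawned.
; Player pickup looks up a data table row by character and arrow tag, spawns attack items, then applies UI and arc settings and refreshes bow ammo count.
; Deletion is skipped for unlimited arrows (inventory value -1).
; Initialization and unequip add small random yaw and sideways offsets, with a helper to reverse them.
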(event EventBeginPlay
  (bind _arrowclass (Variables|UltimateCharacter|GetArrowClass))
  ;[1 1 1] Set item tag and don't allow respawn
  (if (Utilities|IsValidClass _arrowclass)
    (Variables|Default|SetItemTag (Utilities|Struct|BreakFProjectileWeaponData (.ProjectileConfig (Utilities|GetClassDefaults _arrowclass))))
    (else
      (CallFunction|DebugMessage "Base_Arrow_ItemBP" "BeginPlay" "Arrow class is not valid" "NewEnumerator3")))
  (|CallParentFunction)
  (Variables|Default|SetbAllowRespawn false))

(event EventUnequipItem
  ;[1 1 1] Override unequip
  (|CallParentFunction)
  (Internal|AddOffset))

(event EventInitializeConfig
  (params (InConfig :type T%20Attack%20Item%20Struct%20Structure))
  ;[1 1 1] Override initialize config
  (|CallParentFunction InConfig)
  ;[1 1 1] Override unequip
  (Internal|AddOffset))

(event EventEquipItem
  (|CallParentFunction))

(event EventUse
  (|CallParentFunction)
  (CallFunction|UseOverride))

(event EventDeleteItem
  (bind _returnvalue (Game|GetInstigator))
  ;[1 1 1] Don't need to delete unlimit reusable attack items
  (Utilities|IsValid _returnvalue
    (:Is%20Valid
      (bind _asbase_character_bp (Utilities|Casting|CastToBaseCharacter_BP _returnvalue)
        (:then
          (if (.ReturnValue (Utilities|Map|Find (Variables|/Game/UltimateCharacter/Blueprints/Characters/BaseCharacter_BP.BaseCharacter_BP_C|GetArrowsInventory _asbase_character_bp) (Variables|Default|GetItemTag)))
            (if (!= (.Value (Utilities|Map|Find (Variables|/Game/UltimateCharacter/Blueprints/Characters/BaseCharacter_BP.BaseCharacter_BP_C|GetArrowsInventory _asbase_character_bp) (Variables|Default|GetItemTag))) -1)
              (|CallParentFunction))
            (else
              (|CallParentFunction))))
        (:CastFailed
          (|CallParentFunction))))
    (:Is%20Not%20Valid
      (|CallParentFunction))))

(fn ConstructionScript
  (|CallParentFunction)
  (Variables|Default|SetItemType "NewEnumerator6"))

(fn UseOverride
  (CallFunction|DebugMessage "Base_Arrow_ItemBP" "UseOverride" (Utilities|String|ToString(Name) (Variables|Default|GetItemTag)) "NewEnumerator0"))

(fn SetArc
  (params (bInArc :type Boolean))
  (CallFunction|DebugMessage "Base_Arrow_ItemBP" "SetArc" (Utilities|String|ToString(Name) (Variables|Default|GetItemTag)) "NewEnumerator0")
  (Variables|Internal|SetbShowArc bInArc))

(fn GetShowArc
  (return (Variables|Internal|GetbShowArc)))

(fn HasValidClass
  (return (Utilities|IsValidClass (Variables|UltimateCharacter|GetArrowClass))))

(fn PickupItemforPlayer
  (bind _itemtag (Variables|Default|GetItemTag))
  (bind _charactertarget (Variables|Default|GetCharacterTarget))
  (bind _charactertarget_2 (Variables|Default|GetCharacterTarget))
  (bind _arrowsinventory (Variables|/Game/UltimateCharacter/Blueprints/Characters/BaseCharacter_BP.BaseCharacter_BP_C|GetArrowsInventory _charactertarget))
  (bind _equippedweapons (Variables|/Game/UltimateCharacter/Blueprints/Characters/BaseCharacter_BP.BaseCharacter_BP_C|GetEquippedWeapons _charactertarget_2))
  (bind (_value _returnvalue) (Utilities|Map|Find _arrowsinventory _itemtag))
  (bind _output (Utilities|Array|Get(acopy) _equippedweapons))
  (CallFunction|DebugMessage "Base_Arrow_ItemBP" "PickupItemForPlayer" (Utilities|String|ToString(Name) (Variables|Default|GetItemTag)) "NewEnumerator0")
  (Utilities|IsValid (Variables|Default|GetCharacterTarget)
    (:Is%20Valid
      (bind _returnvalue_2 (Utilities|GetDataTableRow "/Game/UltimateCharacter/Blueprints/Data/Tables/Player/T_Player_Arrow.T_Player_Arrow" (Utilities|String|StringToName (Utilities|String|Append (Utilities|String|ToString(Name) (Variables|/Game/UltimateCharacter/Blueprints/Characters/BaseCharacter_BP.BaseCharacter_BP_C|GetCharacterTag (Variables|Default|GetCharacterTarget))) (Utilities|String|ToString(Name) (Variables|Default|GetItemTag)))))
        (:then
          ;[1 1 1] Spawn arrow & initialize for player
          (bind _outitemindex (Default|SpawnAttackItems (Variables|Default|GetCharacterTarget) (Utilities|Struct|BreakT_Arrow_Struct (.Base (Utilities|Struct|BreakT_PlayerArrow_Struct _returnvalue_2))) (select _returnvalue _value (Utilities|Map|Length _arrowsinventory)) (Variables|Default|GetItemTag) (Utilities|GetClass self)))
          (LocalVariables|SetTempOutIndex _outitemindex)
          (if (> (LocalVariables|GetTempOutIndex) -1)
            (Default|InitializeforPlayer (Utilities|Array|Get(acopy) (Variables|/Game/UltimateCharacter/Blueprints/Characters/BaseCharacter_BP.BaseCharacter_BP_C|GetAttackItems (Variables|Default|GetCharacterTarget)) (LocalVariables|GetTempOutIndex)) (.UI (Utilities|Struct|BreakT_PlayerArrow_Struct _returnvalue_2)))
            (bind _asbase_arrow_item_bp (Utilities|Casting|CastToBase_Arrow_ItemBP (Utilities|Array|Get(acopy) (Variables|/Game/UltimateCharacter/Blueprints/Characters/BaseCharacter_BP.BaseCharacter_BP_C|GetAttackItems (Variables|Default|GetCharacterTarget)) (LocalVariables|GetTempOutIndex)))
              (:then
                (Arc|SetArc _asbase_arrow_item_bp (.bShowArc (Utilities|Struct|BreakT_PlayerArrow_Struct _returnvalue_2))))
              (:CastFailed
                _))
            (Utilities|IsValid _output
              (:Is%20Valid
                (bind _asbase_bow_bp (Utilities|Casting|CastToBaseBow_BP _output)
                  (:then
                    (Default|UpdateArrowCountUI (Variables|Default|GetCharacterTarget) (Variables|Default|GetItemTag) (Variables|/Game/UltimateCharacter/Blueprints/Weapons/BaseWeapon_BP.BaseWeapon_BP_C|GetWeaponTag _asbase_bow_bp)))
                  (:CastFailed
                    _)))
              (:Is%20Not%20Valid
                _))
            (return true)
            (else
              (CallFunction|DebugMessage "Base_Arrow_ItemBP" "PickupItemForPlayer" (Utilities|String|Append (Utilities|String|ToString(Name) (Variables|Default|GetItemTag)) " Failed, index is not valid.") "NewEnumerator2")
              (return false))))
        (:RowNotFound
          (CallFunction|DebugMessage "Base_Arrow_ItemBP" "PickupItemForPlayer" (Utilities|String|Append (Utilities|String|ToString(Name) (Variables|Default|GetItemTag)) " not found in table for " (Utilities|String|ToString(Name) (Variables|/Game/UltimateCharacter/Blueprints/Characters/BaseCharacter_BP.BaseCharacter_BP_C|GetCharacterTag (Variables|Default|GetCharacterTarget)))) "NewEnumerator2")
          (Default|HUDMessage (Variables|Default|GetCharacterTarget) "You're not allowed to pick up this arrow item!" "NewEnumerator0")
          (return false))))
    (:Is%20Not%20Valid
      (CallFunction|DebugMessage "Base_Arrow_ItemBP" "PickupItemForPlayer" "Character target is not valid" "NewEnumerator2")
      (return false))))

(fn AddOffset
  (CallFunction|DebugMessage "Base_Arrow_ItemBP" "AddRotationOffset" "" "NewEnumerator0")
  ;[1 1 1] Add offset to the actor
  (Variables|Internal|SetOffsetYaw (Math|Random|RandomFloatinRange -5.0 5.0))
  (Transformation|AddActorLocalRotation (Math|Rotator|MakeRotator 0.0 0.0 (Variables|Internal|GetOffsetYaw)) false false)
  (Variables|Internal|SetOffsetY (Math|Random|RandomFloatinRange -2.0 2.0))
  (Transformation|AddActorLocalOffset (Math|Vector|MakeVector 0.0 (Variables|Internal|GetOffsetY) 0.0) false false))

(fn RemoveOffset
  (CallFunction|DebugMessage "Base_Arrow_ItemBP" "RemoveOffset" "" "NewEnumerator0")
  ;[1 1 1] Remove offset from the actor
  (Transformation|AddActorLocalRotation (Math|Rotator|MakeRotator 0.0 0.0 (* (Variables|Internal|GetOffsetYaw) -1.0)) false false)
  (Transformation|AddActorLocalOffset (Math|Vector|MakeVector 0.0 (* (Variables|Internal|GetOffsetY) -1.0) 0.0) false false))