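; Base weapon pickup that spawns a gun or melee weapon for the character picking it up.
; BeginPlay takes the item tag from the weapon class defaults, and OnPickup validates it before routing to player or AI handling.
; For players, character tag plus item tag keys a gun or melee data table row used to spawn and initialize the weapon; missing rows deny pickup with a HUD message.
; AI pickup is an unimplemented stub that always fails.
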(event EventOnPickup
  (params (InCharacter :type Base%20Character%20BP%20Object%20Reference))
  ;[1 1 1] Run pickup function on Player or AI
  (bind _output_get (Variables|Internal|SetCharacterTarget InCharacter))
  (Utilities|IsValid _output_get
    (:Is%20Valid
      (if (Utilities|Name|NotEqual(Name) (Variables|Default|GetItemTag) "None")
        (if (Utilities|IsValidClass (Variables|UltimateCharacter|GetWeaponClass))
          (bind _asplayer_character_bp (Utilities|Casting|CastToPlayerCharacter_BP (Variables|Internal|GetCharacterTarget))
            (:then
              (bind _boutvaliditem (CallFunction|PickupforPlayer _asplayer_character_bp))
              (if _boutvaliditem
                (|CallParentFunction (Variables|Internal|GetCharacterTarget) :!label _label)))
            (:CastFailed
              (bind _asaicharacter_bp (Utilities|Casting|CastToAICharacter_BP (Variables|Internal|GetCharacterTarget))
                (:then
                  (bind _boutvaliditem_2 (CallFunction|PickupforAI _asaicharacter_bp))
                  (if _boutvaliditem_2
                    (goto _label)))
                (:CastFailed
                  (CallFunction|DebugMessage "BaseWeapon_Pickup_BP" "OnPickup" "Character cast failed" "NewEnumerator2")))))
          (else
            (CallFunction|DebugMessage "BaseWeapon_Pickup_BP" "OnPickup" "Weapon class is not valid" "NewEnumerator2")))
        (else
          (CallFunction|DebugMessage "BaseWeapon_Pickup_BP" "OnPickup" "Item tag is 'None', Try to set PickUp tag if you put this directly in level" "NewEnumerator2"))))
    (:Is%20Not%20Valid
      (CallFunction|DebugMessage "BaseWeapon_Pickup_BP" "OnPickup" (Utilities|String|Append "Character is not valid to pickup " (Utilities|GetDisplayName self)) "NewEnumerator2"))))

(event Collision|EventActorBeginOverlap
  (params (OtherActor :type Actor%20Object%20Reference))
  (|CallParentFunction OtherActor) ; This node is disabled and will not be called.\nDrag off pins to build functionality.
)

(event EventTick
  (params (DeltaSeconds :type Float%20%28single-precision%29))
  (|CallParentFunction DeltaSeconds) ; This node is disabled and will not be called.\nDrag off pins to build functionality.
)

(event EventBeginPlay
  ;[1 1 1] Set item tag from weapon base class
  (Variables|Default|SetItemTag (.WeaponTag (Utilities|GetClassDefaults (Variables|UltimateCharacter|GetWeaponClass))))
  (|CallParentFunction))

(fn ConstructionScript
  (|CallParentFunction))

(fn PickupforPlayer
  (params (InPlayer :type Player%20Character%20BP%20Object%20Reference))
  (bind _itemtag (Variables|Default|GetItemTag))
  (bind _itemtag_2 (Variables|Default|GetItemTag))
  (bind _itemtag_3 (Variables|Default|GetItemTag))
  (bind _itemtag_4 (Variables|Default|GetItemTag))
  (bind _returnvalue (Utilities|String|ToString(Name) _itemtag_4))
  (bind _returnvalue_2 (Utilities|String|ToString(Name) _itemtag))
  (bind _returnvalue_3 (Utilities|String|ToString(Name) _itemtag_3))
  (bind _returnvalue_4 (Utilities|String|ToString(Name) _itemtag_2))
  (bind _charactertag (Variables|/Game/UltimateCharacter/Blueprints/Characters/BaseCharacter_BP.BaseCharacter_BP_C|GetCharacterTag InPlayer))
  (bind _charactertag_2 (Variables|/Game/UltimateCharacter/Blueprints/Characters/BaseCharacter_BP.BaseCharacter_BP_C|GetCharacterTag InPlayer))
  (bind _charactertag_3 (Variables|/Game/UltimateCharacter/Blueprints/Characters/BaseCharacter_BP.BaseCharacter_BP_C|GetCharacterTag InPlayer))
  (bind _charactertag_4 (Variables|/Game/UltimateCharacter/Blueprints/Characters/BaseCharacter_BP.BaseCharacter_BP_C|GetCharacterTag InPlayer))
  (bind _returnvalue_5 (Utilities|String|ToString(Name) _charactertag))
  (bind _returnvalue_6 (Utilities|String|ToString(Name) _charactertag_4))
  (bind _returnvalue_7 (Utilities|String|ToString(Name) _charactertag_3))
  (bind _returnvalue_8 (Utilities|String|ToString(Name) _charactertag_2))
  (bind _returnvalue_9 (Utilities|String|Append _returnvalue_5 _returnvalue_2))
  (bind _returnvalue_10 (Utilities|String|Append _returnvalue_7 _returnvalue_4))
  ;[1 1 1] Get gun data from table
  (CallFunction|DebugMessage "BaseWeapon_Pickup_BP" "PickupForPlayer" (Utilities|String|Append "Pickup: " (Utilities|String|ToString(Name) (Variables|Default|GetItemTag)) " for " (Utilities|String|ToString(Name) (Variables|/Game/UltimateCharacter/Blueprints/Characters/BaseCharacter_BP.BaseCharacter_BP_C|GetCharacterTag InPlayer))) "NewEnumerator0")
  (if (Utilities|ClassIsChildOf (Variables|UltimateCharacter|GetWeaponClass) "/Game/UltimateCharacter/Blueprints/Weapons/Guns/BaseGun_BP.BaseGun_BP_C")
    (bind _returnvalue_11 (Utilities|GetDataTableRow "/Game/UltimateCharacter/Blueprints/Data/Tables/Player/T_Player_Gun.T_Player_Gun" (Utilities|String|StringToName _returnvalue_10))
      (:then
        ;[1 1 1] Spawn & initialize gun
        (bind (_boutspawned _outgun) (Default|SpawnGun InPlayer (.BaseGun (Utilities|Struct|BreakT_PlayerGun_Struct _returnvalue_11))))
        (LocalVariables|SetTempWeapon _outgun)
        (if _boutspawned
          (CallFunction|DebugMessage "BaseWeapon_Pickup_BP" "PickupForPlayer" (Utilities|String|Append _returnvalue " spawned for " _returnvalue_6) "NewEnumerator0")
          (bind _asbase_gun_bp (Utilities|Casting|CastToBaseGun_BP (LocalVariables|GetTempWeapon))
            (:then
              (Default|SetShowArc _asbase_gun_bp (.bShowArc (Utilities|Struct|BreakT_PlayerGun_Struct _returnvalue_11)))
              (Default|InitializeFPGunAnimations _asbase_gun_bp (.GunFirsPersonAnimation (Utilities|Struct|BreakT_PlayerGun_Struct _returnvalue_11)))
              (Default|InitializeforPlayer (LocalVariables|GetTempWeapon) (.UI (Utilities|Struct|BreakT_PlayerGun_Struct _returnvalue_11)) (.WeaponFirstPersonAnimation (Utilities|Struct|BreakT_PlayerGun_Struct _returnvalue_11)) (.CameraConfig (Utilities|Struct|BreakT_PlayerGun_Struct _returnvalue_11)))
              (return true))
            (:CastFailed
              (CallFunction|DebugMessage "BaseWeapon_Pickup_BP" "PickupForPlayer" "Cast to gun failed" "NewEnumerator2")
              (return false)))
          (else
            (CallFunction|DebugMessage "BaseWeapon_Pickup_BP" "PickupForPlayer" (Utilities|String|Append _returnvalue " spawn failed for " _returnvalue_6) "NewEnumerator2")
            (return false))))
      (:RowNotFound
        (CallFunction|DebugMessage "BaseWeapon_Pickup_BP" "PickupForPlayer" (Utilities|String|Append _returnvalue_10 " not found in T_Player_Gun") "NewEnumerator2")
        (Default|HUDMessage InPlayer "You're not allowed to pickup guns." "NewEnumerator2")
        (return false)))
    (elif (Utilities|ClassIsChildOf (Variables|UltimateCharacter|GetWeaponClass) "/Game/UltimateCharacter/Blueprints/Weapons/Melee/BaseMelee_BP.BaseMelee_BP_C")
      ;[1 1 1] Get sword data from table
      (bind _returnvalue_12 (Utilities|GetDataTableRow "/Game/UltimateCharacter/Blueprints/Data/Tables/Player/T_Player_Melee.T_Player_Melee" (Utilities|String|StringToName _returnvalue_9))
        (:then
          ;[1 1 1] Spawn & initialize sword
          (bind (_boutspawned_2 _outsword) (Default|SpawnMelee InPlayer (.BaseMelee (Utilities|Struct|BreakT_PlayerMelee_Struct _returnvalue_12))))
          (LocalVariables|SetTempWeapon _outsword)
          (if _boutspawned_2
            (CallFunction|DebugMessage "BaseWeapon_Pickup_BP" "PickupForPlayer" (Utilities|String|Append _returnvalue_3 " spawned for " _returnvalue_8) "NewEnumerator0")
            (Default|InitializeforPlayer (LocalVariables|GetTempWeapon) (.UI (Utilities|Struct|BreakT_PlayerMelee_Struct _returnvalue_12)) (.WeaponFirstPersonAnimation (Utilities|Struct|BreakT_PlayerMelee_Struct _returnvalue_12)) (.CameraConfig (Utilities|Struct|BreakT_PlayerMelee_Struct _returnvalue_12)))
            (return true)
            (else
              (CallFunction|DebugMessage "BaseWeapon_Pickup_BP" "PickupForPlayer" (Utilities|String|Append _returnvalue_3 " spawn failed for " _returnvalue_8) "NewEnumerator2")
              (return false))))
        (:RowNotFound
          (CallFunction|DebugMessage "BaseWeapon_Pickup_BP" "PickupForPlayer" (Utilities|String|Append _returnvalue_9 " not found in T_Player_Sword") "NewEnumerator2")
          (Default|HUDMessage InPlayer "You're not allowed to pickup swords." "NewEnumerator2")
          (return false)))
      (else
        (CallFunction|DebugMessage "BaseWeapon_Pickup_BP" "PickupForPlayer" (Utilities|String|Append (Utilities|GetClassDisplayName (Variables|UltimateCharacter|GetWeaponClass)) " cast failed!") "NewEnumerator2")
        (return false)))))

(fn PickupforAI
  (params (InAI :type AI%20Character%20BP%20Object%20Reference))
  (CallFunction|DebugMessage "BaseWeapon_Pickup_BP" "OnPickup" (Utilities|String|Append "TODO: " "Pickup " (Utilities|String|ToString(Name) (Variables|Default|GetItemTag)) " for " (Utilities|String|ToString(Name) (Variables|/Game/UltimateCharacter/Blueprints/Characters/BaseCharacter_BP.BaseCharacter_BP_C|GetCharacterTag InAI))) "NewEnumerator0")
  (return false))