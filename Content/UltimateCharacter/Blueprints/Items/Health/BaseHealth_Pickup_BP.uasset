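; Base health pickup item that heals the character picking it up by its Health amount.
; BeginPlay registers it as an AI sight stimulus source so AI perception can see it.
; OnPickup validates the character, calls HealCharacter and then the parent pickup logic, or logs a debug message if invalid.
; Pickup on mesh overlap is present but left disconnected, so healing happens only through the pickup command.
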(event OnComponentBeginOverlap(Mesh)
  (params (OverlappedComponent :type Primitive%20Component%20Object%20Reference) (OtherActor :type Actor%20Object%20Reference) (OtherComp :type Primitive%20Component%20Object%20Reference) (OtherBodyIndex :type Integer) (bFromSweep :type Boolean) (SweepResult :type Hit%20Result%20Structure%20%28by%20ref%29))
  ;[1 1 1] Overlap pickup is not activated you can activate by connecting nodes
)

(event EventBeginPlay
  (|CallParentFunction)
  (Class|AIPerceptionSystem|RegisterPerceptionStimuliSource "/Script/AIModule.AISense_Sight" self))

(event Collision|EventActorBeginOverlap
  (params (OtherActor :type Actor%20Object%20Reference)))

(event EventTick
  (params (DeltaSeconds :type Float%20%28single-precision%29))
  (|CallParentFunction DeltaSeconds) ; This node is disabled and will not be called.\nDrag off pins to build functionality.
)

(event EventOnPickup
  (params (InCharacter :type Base%20Character%20BP%20Object%20Reference))
  ;[1 1 1] Pickup item when pickup command received
  (bind _output_get (Variables|Internal|SetCharacterTarget InCharacter))
  (Utilities|IsValid _output_get
    (:Is%20Valid
      (Default|HealCharacter (Variables|Internal|GetCharacterTarget) (Variables|UltimateCharacter|GetHealth))
      (|CallParentFunction (Variables|Internal|GetCharacterTarget)))
    (:Is%20Not%20Valid
      (CallFunction|DebugMessage "BaseAmmo_Pickup_BP" "OnPickup" (Utilities|String|Append "Character is not valid to pickup " (Utilities|String|ToString(Name) (Variables|Default|GetItemTag))) "NewEnumerator0"))))

(fn ConstructionScript
  (|CallParentFunction))