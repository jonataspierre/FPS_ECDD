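; Base throw item that characters pick up and use to launch projectiles, taking its tag from the projectile class defaults.
; Pickup looks up T_Player_Throw by character and item tag, then spawns and initializes an attack item with UI, first-person animation and arc flag.
; Use spawns Count projectiles at the attach socket, offset to alternating sides.
; Deletion is skipped when the instigator's ThrowsInventory value is -1, marking reusable unlimited throws.
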(event EventBeginPlay
  ;[1 1 1] Set item tag and don't allow respawn
  (Variables|Default|SetItemTag (Utilities|Struct|BreakFProjectileWeaponData (.ProjectileConfig (Utilities|GetClassDefaults (Variables|UltimateCharacter|GetProjectileClass)))))
  (|CallParentFunction)
  (Variables|Default|SetbAllowRespawn false))

(event Collision|EventActorBeginOverlap
  (params (OtherActor :type Actor%20Object%20Reference))
  (|CallParentFunction OtherActor) ; This node is disabled and will not be called.\nDrag off pins to build functionality.
)

(event EventTick
  (params (DeltaSeconds :type Float%20%28single-precision%29))
  (|CallParentFunction DeltaSeconds) ; This node is disabled and will not be called.\nDrag off pins to build functionality.
)

(event EventUse
  (|CallParentFunction)
  (Interact|UseOverride))

(event EventDeleteItem
  (bind _returnvalue (Game|GetInstigator))
  ;[1 1 1] Don't need to delete unlimit reusable attack items, for example narbash can throw his mace unlimited
  (Utilities|IsValid _returnvalue
    (:Is%20Valid
      (bind _asbase_character_bp (Utilities|Casting|CastToBaseCharacter_BP _returnvalue)
        (:then
          (if (.ReturnValue (Utilities|Map|Find (Variables|/Game/UltimateCharacter/Blueprints/Characters/BaseCharacter_BP.BaseCharacter_BP_C|GetThrowsInventory _asbase_character_bp) (Variables|Default|GetItemTag)))
            (if (!= (.Value (Utilities|Map|Find (Variables|/Game/UltimateCharacter/Blueprints/Characters/BaseCharacter_BP.BaseCharacter_BP_C|GetThrowsInventory _asbase_character_bp) (Variables|Default|GetItemTag))) -1)
              (|CallParentFunction))
            (else
              (|CallParentFunction))))
        (:CastFailed
          (|CallParentFunction))))
    (:Is%20Not%20Valid
      (|CallParentFunction))))

(fn ConstructionScript
  (|CallParentFunction)
  (Variables|Default|SetItemType "NewEnumerator3"))

(fn UseOverride
  (bind _returnvalue (Game|GetInstigator))
  (bind _itemconfig (Variables|Default|GetItemConfig))
  (bind _attachsocket (Utilities|Struct|BreakT_AttackItem_Struct _itemconfig))
  (CallFunction|DebugMessage "Base_Throw_Pickup_BP" "UseOverride" (Utilities|String|ToString(Name) (Variables|Default|GetItemTag)) "NewEnumerator0")
  (bind _asbase_character_bp (Utilities|Casting|CastToBaseCharacter_BP (Game|GetInstigator))
    (:then
      (Variables|Internal|SetbPendingThrow true)
      (for _index (range 0 (- (Variables|Default|GetCount) 1))
        ;[1 1 1] Spawn & init projectile velocity
        (bind _returnvalue_2 (Game|SpawnActorfromClass (Variables|UltimateCharacter|GetProjectileClass) (Math|Transform|MakeTransform (+ (Transformation|GetSocketLocation (Default|GetMesh _asbase_character_bp) _attachsocket) (* (Transformation|GetActorRightVector (Game|GetInstigator)) (* _index (Math|Float|SelectFloat 1e+02 -1e+02 (== (Math|Integer|%(Integer) _index 2) 0))))) (Transformation|GetSocketRotation (Default|GetMesh _asbase_character_bp) _attachsocket)) "AdjustIfPossibleButAlwaysSpawn" "SelectDefaultAtRuntime" _returnvalue _returnvalue))
        (Default|InitVelocity _returnvalue_2))
      (Variables|Default|SetCount 0))
    (:CastFailed
      (CallFunction|DebugMessage "Base_Throw_Pickup_BP" "UseOverride" "Instigator is not child of BaseCharacter" "NewEnumerator2"))))

(fn HasValidClass
  (return (Utilities|IsValidClass (Variables|UltimateCharacter|GetProjectileClass))))

(fn PickupItemforPlayer
  (bind _itemtag (Variables|Default|GetItemTag))
  (bind _charactertarget (Variables|Default|GetCharacterTarget))
  (bind _throwsinventory (Variables|/Game/UltimateCharacter/Blueprints/Characters/BaseCharacter_BP.BaseCharacter_BP_C|GetThrowsInventory _charactertarget))
  (bind (_value _returnvalue) (Utilities|Map|Find _throwsinventory _itemtag))
  (CallFunction|DebugMessage "Base_ThrowItemBP" "PickupItemForPlayer" (Utilities|String|ToString(Name) (Variables|Default|GetItemTag)) "NewEnumerator0")
  (Utilities|IsValid (Variables|Default|GetCharacterTarget)
    (:Is%20Valid
      ;[1 1 1] Read data from table
      (bind _returnvalue_2 (Utilities|GetDataTableRow "/Game/UltimateCharacter/Blueprints/Data/Tables/Player/T_Player_Throw.T_Player_Throw" (Utilities|String|StringToName (Utilities|String|Append (Utilities|String|ToString(Name) (Variables|/Game/UltimateCharacter/Blueprints/Characters/BaseCharacter_BP.BaseCharacter_BP_C|GetCharacterTag (Variables|Default|GetCharacterTarget))) (Utilities|String|ToString(Name) (Variables|Default|GetItemTag)))))
        (:then
          ;[1 1 1] Spawn throws & initialize for player
          (bind _outitemindex (Default|SpawnAttackItems (Variables|Default|GetCharacterTarget) (Utilities|Struct|BreakT_Throw_Struct (.Base (Utilities|Struct|BreakT_PlayerThrow_Struct _returnvalue_2))) (select _returnvalue _value (Utilities|Map|Length _throwsinventory)) (Variables|Default|GetItemTag) (Utilities|GetClass self)))
          (LocalVariables|SetTempOutIndex _outitemindex)
          (if (> (LocalVariables|GetTempOutIndex) -1)
            (Default|InitializeforPlayer (Utilities|Array|Get(acopy) (Variables|/Game/UltimateCharacter/Blueprints/Characters/BaseCharacter_BP.BaseCharacter_BP_C|GetAttackItems (Variables|Default|GetCharacterTarget)) (LocalVariables|GetTempOutIndex)) (.UI (Utilities|Struct|BreakT_PlayerThrow_Struct _returnvalue_2)) (.FirstPersonAnimation (Utilities|Struct|BreakT_PlayerThrow_Struct _returnvalue_2)))
            (bind _asbase_throw_item_bp (Utilities|Casting|CastToBase_ThrowItemBP (Utilities|Array|Get(acopy) (Variables|/Game/UltimateCharacter/Blueprints/Characters/BaseCharacter_BP.BaseCharacter_BP_C|GetAttackItems (Variables|Default|GetCharacterTarget)) (LocalVariables|GetTempOutIndex))))
            (Arc|SetArc _asbase_throw_item_bp (.bShowArc (Utilities|Struct|BreakT_PlayerThrow_Struct _returnvalue_2)))
            (return true)
            (else
              (CallFunction|DebugMessage "Base_Bombard_Pickup_BP" "PickupItemForPlayer" (Utilities|String|Append (Utilities|String|ToString(Name) (Variables|Default|GetItemTag)) " Failed, index is not valid.") "NewEnumerator2")
              (return false))))
        (:RowNotFound
          (CallFunction|DebugMessage "Base_ThrowItemBP" "PickupItemForPlayer" (Utilities|String|Append (Utilities|String|ToString(Name) (Variables|Default|GetItemTag)) " not found in table") "NewEnumerator2")
          (Default|HUDMessage (Variables|Default|GetCharacterTarget) "You're not allwoed to pick up this throw item!" "NewEnumerator0")
          (return false))))
    (:Is%20Not%20Valid
      (CallFunction|DebugMessage "Base_ThrowItemBP" "PickupItemForPlayer" "Character target is not valid!" "NewEnumerator2")
      (return false))))

(fn SetArc
  (params (bInArc :type Boolean))
  (CallFunction|DebugMessage "Base_ThrowItemBP" "SetArc" (Utilities|String|ToString(Name) (Variables|Default|GetItemTag)) "NewEnumerator0")
  (Variables|Internal|SetbShowArc bInArc))

(fn GetShowArc
  (return (Variables|Internal|GetbShowArc)))