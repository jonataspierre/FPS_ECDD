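; Base blueprint for attack items that characters carry, equip and use, with item config set up separately for AI and player owners.
; OnPickup accepts only player characters, gated by HasValidClass and PickupItemForPlayer, stubs returning false here; overlap pickup is left unwired.
; Equip and unequip snap the item to hand or inventory sockets on the instigator's mesh.
; Use emits sound, AI noise and camera shake; BeginPlay strips pickup physics and effects from owned, non-dropped items.
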(event OnComponentBeginOverlap(Mesh)
  (params (OverlappedComponent :type Primitive%20Component%20Object%20Reference) (OtherActor :type Actor%20Object%20Reference) (OtherComp :type Primitive%20Component%20Object%20Reference) (OtherBodyIndex :type Integer) (bFromSweep :type Boolean) (SweepResult :type Hit%20Result%20Structure%20%28by%20ref%29))
  ;[1 1 1] Overlap pickup is not activated you can activate by connecting nodes
)

(event EventUse
  (bind _returnvalue (Game|GetInstigator))
  (bind _usingsound (Variables|UltimateCharacter|GetUsingSound))
  (bind (_sound _noise) (Utilities|Struct|BreakFBaseSound _usingsound))
  (|CallParentFunction)
  ;[1 1 1] Play using item sound
  (bind _asbase_character_bp (Utilities|Casting|CastToBaseCharacter_BP _returnvalue))
  (Default|MakePawnNoise _asbase_character_bp _noise)
  (Audio|PlaySoundatLocation _sound (Transformation|GetActorLocation _returnvalue) "0, 0, 0" 1.0 1.0 0.0 0 0 0 0)
  ;[1 1 1] Play camera shake
  (Utilities|IsValid (Game|GetInstigatorController)
    (:Is%20Valid
      (bind _asplayer_controller (Utilities|Casting|CastToPlayerController (Game|GetInstigatorController)))
      (Game|Feedback|ClientStartCameraShake _asplayer_controller (Variables|UltimateCharacter|GetCameraShake) 1.0 "CameraLocal" "0, 0, 0"))))

(event Collision|EventActorBeginOverlap
  (params (OtherActor :type Actor%20Object%20Reference))
  (|CallParentFunction OtherActor) ; This node is disabled and will not be called.\nDrag off pins to build functionality.
)

(event EventTick
  (params (DeltaSeconds :type Float%20%28single-precision%29))
  (|CallParentFunction DeltaSeconds) ; This node is disabled and will not be called.\nDrag off pins to build functionality.
)

(event EventOnPickup
  (params (InCharacter :type Base%20Character%20BP%20Object%20Reference))
  ;[1 1 1] Check attack item for pickup
  (Variables|Internal|SetCharacterTarget InCharacter)
  (Utilities|IsValid (Variables|Internal|GetCharacterTarget)
    (:Is%20Valid
      (if (Utilities|Name|NotEqual(Name) (Variables|Default|GetItemTag) "None")
        (bind _boutvalid (Internal|HasValidClass))
        ;[1 1 1] Only players can pickup attack items
        (if _boutvalid
          (if (Utilities|ClassIsChildOf (Utilities|GetClass (Variables|Internal|GetCharacterTarget)) "/Game/UltimateCharacter/Blueprints/Characters/PlayerCharacter_BP.PlayerCharacter_BP_C")
            (bind _boutvaliditem (Internal|PickupItemforPlayer))
            (if _boutvaliditem
              (CallFunction|DisableCollisionandPhysics)
              (|CallParentFunction (Variables|Internal|GetCharacterTarget))
              (else
                (CallFunction|DebugMessage "Base_AttackItemBP" "OnPickup" "Player can't pickup item!" "NewEnumerator2"))))
          (else
            (CallFunction|DebugMessage "Base_AttackItemBP" "OnPickup" "Has not a valid class!" "NewEnumerator3")))
        (else
          (CallFunction|DebugMessage "Base_AttackItemBP" "OnPickup" "Item tag is 'None'" "NewEnumerator3"))))
    (:Is%20Not%20Valid
      (CallFunction|DebugMessage "Base_AttackItemBP" "OnPickup" (Utilities|String|Append "Character is not valid to pickup " (Utilities|GetDisplayName self)) "NewEnumerator3"))))

(event EventBeginPlay
  (|CallParentFunction)
  (Initialize|CheckVisibility))

(fn ConstructionScript
  (|CallParentFunction))

(fn InitializeConfig
  (params (InConfig :type T%20Attack%20Item%20Struct%20Structure))
  (CallFunction|DebugMessage "Base_AttackItem_BP" "InitializeConfig" (Utilities|String|ToString(Name) (Variables|Default|GetItemTag)) "NewEnumerator0")
  ;[1 1 1] Set item config and attach to inventory of character
  (bind _output_get (Variables|Internal|SetItemConfig InConfig))
  (bind _asbase_character_bp (Utilities|Casting|CastToBaseCharacter_BP (Game|GetInstigator)))
  (Transformation|AttachComponentToComponent (Default|GetMesh _asbase_character_bp) (Utilities|Array|Get(acopy) (Utilities|Struct|BreakT_AttackItem_Struct _output_get)) "SnapToTarget" "SnapToTarget" "SnapToTarget" true))

(fn InitializeforAI
  (params (Distance :type Float%20Range%20Structure))
  (CallFunction|DebugMessage "Base_AttackItem_BP" "InitializeForAI" (Utilities|String|ToString(Name) (Variables|Default|GetItemTag)) "NewEnumerator0")
  ;[1 1 1] Initialize item for AI characters
  (Variables|Internal|SetDistance Distance))

(fn InitializeforPlayer
  (params (InUI :type Base%20UMG%20Struct%20Structure) (InFPAnimation :type F%20Animation%20Info%20Structure) (InCameraConfig :type T%20Player%20Camera%20Struct%20Structure))
  (CallFunction|DebugMessage "Base_AttackItem_BP" "InitializeForPlayer" (Utilities|String|ToString(Name) (Variables|Default|GetItemTag)) "NewEnumerator0")
  ;[1 1 1] Initialize item for player characters
  (Variables|Internal|SetUIConfig InUI)
  (Variables|Internal|SetFirstPersonAnimation InFPAnimation)
  (Variables|Internal|SetCameraConfig InCameraConfig))

(fn EquipItem
  ;[1 1 1] Try to attach item to character
  (CallFunction|DebugMessage "Base_AttackItem_BP" "Equip" (Utilities|String|ToString(Name) (Variables|Default|GetItemTag)) "NewEnumerator0")
  (bind _asbase_character_bp (Utilities|Casting|CastToBaseCharacter_BP (Game|GetInstigator)))
  (Transformation|AttachComponentToComponent (Default|GetMesh _asbase_character_bp) (Utilities|Struct|BreakT_AttackItem_Struct (Variables|Internal|GetItemConfig)) "SnapToTarget" "SnapToTarget" "KeepWorld" true))

(fn UnequipItem
  (CallFunction|DebugMessage "Base_AttackItem_BP" "Unequip" (Utilities|String|ToString(Name) (Variables|Default|GetItemTag)) "NewEnumerator0")
  ;[1 1 1] Unequip item & attach to inventory
  (bind _asbase_character_bp (Utilities|Casting|CastToBaseCharacter_BP (Game|GetInstigator)))
  (Transformation|AttachComponentToComponent (Default|GetMesh _asbase_character_bp) (Utilities|Array|Get(acopy) (Utilities|Struct|BreakT_AttackItem_Struct (Variables|Internal|GetItemConfig))) "SnapToTarget" "SnapToTarget" "SnapToTarget" true))

(fn DeleteItem
  ;[1 1 1] Disable collsion and delete item
  (CallFunction|DebugMessage "Base_AttackItem_BP" "DeleteItem" (Utilities|String|ToString(Name) (Variables|Default|GetItemTag)) "NewEnumerator0")
  (Collision|SetCollisionEnabled (Variables|Character|GetMesh) "NoCollision")
  (Development|SetHiddeninGame (Variables|Character|GetMesh) true false)
  (Rendering|SetActorHiddenInGame true)
  (Actor|DestroyActor))

(fn HasValidClass
  (return false))

(fn PickupItemforPlayer
  (CallFunction|DebugMessage "Base_AttackItem_BP" "PickupItemForPlayer" (Utilities|String|ToString(Name) (Variables|Default|GetItemTag)) "NewEnumerator0")
  (return false))

(fn CheckVisibility
  (CallFunction|DebugMessage "Base_AttackItem_BP" "CheckVisibility" (Utilities|String|ToString(Name) (Variables|Default|GetItemTag)) "NewEnumerator0")
  (Utilities|IsValid (Game|GetInstigator)
    (:Is%20Valid
      (if (not (Variables|Default|GetbSpawnByDrop))
        ;[1 1 1] Disable physics
        (Physics|SetSimulatePhysics (Variables|Character|GetMesh) false)
        ;[1 1 1] Destroy effect components
        (Components|DestroyComponent (Variables|Default|GetMeshEffect))
        (Components|DestroyComponent (Variables|Default|GetRotatingMovement))
        ;[1 1 1] Dont show attack item for this, when item has instigator
        (if (Variables|UltimateCharacter|GetbHideAfterPickup)
          (Rendering|SetVisibility (Variables|Character|GetMesh) false false))))))

(fn SetCount
  (params (InCount :type Integer))
  (Variables|Internal|SetCount InCount)
  (CallFunction|DebugMessage "Base_AttackItem_BP" "SetCount" (Utilities|String|Append (Utilities|String|ToString(Integer) (Variables|Internal|GetCount)) ", " (Utilities|String|ToString(Name) (Variables|Default|GetItemTag))) "NewEnumerator0"))