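; Base melee weapon (sword) that adapts the parent weapon's fire, burst and ammo flow to swings.
; Timers pace swings and delay player stops, while active combos skip the wait and AI controllers gate attacks.
; While FireSword is set, the locally controlled Tick runs line or box traces, applying block-adjusted damage.
; Ammo acts as uses, spent once per swing on a damageable hit; depleted weapons leave the pawn.
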(event EventBeginPlay
  ;[1 1 1] Set weapon type to sword
  (|CallParentFunction)
  (Variables|Default|SetWeaponType "NewEnumerator3"))

(event Collision|EventActorBeginOverlap
  (params (OtherActor :type Actor%20Object%20Reference))
  (|CallParentFunction OtherActor) ; This node is disabled and will not be called.\nDrag off pins to build functionality.
)

(event EventTick
  (params (DeltaSeconds :type Float%20%28single-precision%29))
  ;[1 1 1] Control firing sword from animation
  (|CallParentFunction DeltaSeconds)
  (Utilities|IsValid (Variables|Default|GetMyPawn)
    (:Is%20Valid
      (if (Math|Boolean|ANDBoolean (Variables|Internal|GetFireSword) (Utilities|Enum|Equal(Enum) (Variables|Default|GetCurrentState) "NewEnumerator1") (Pawn|IsLocallyControlled (Variables|Default|GetMyPawn)))
        (CallFunction|FireWeapon)))))

(event EventOnBurstStarted
  ;[1 1 1] Override OnBurstStarted functio
  (|CallParentFunction)
  (Weapon|OnBurstStartedOverride))

(event EventHandleFiring
  ;[1 1 1] Overrid HandleFiring function
  (|CallParentFunction)
  (Firing|HandlFiringOverride))

(event EventFireWeapon
  ;[1 1 1] Override FireWeapon function
  (Weapon|InternalFireWeapon))

(event EventStopFire
  ;[1 1 1] Override stop fire to customize it for player characters
  (Utilities|IsValid (Variables|Default|GetMyPawn)
    (:Is%20Valid
      (if (Utilities|ClassIsChildOf (Utilities|GetClass (Variables|Default|GetMyPawn)) "/Game/UltimateCharacter/Blueprints/Characters/PlayerCharacter_BP.PlayerCharacter_BP_C")
        (Firing|StopFireOverride)
        (else
          (Ammo|OutOfUseCheck :!label _label)
          (|CallParentFunction))))
    (:Is%20Not%20Valid
      (goto _label))))

(event EventStartFire
  ;[1 1 1] Todo : reseting stop timer needs to call on server too
  (Utilities|Time|ClearandInvalidateTimerbyHandle (Variables|Internal|GetHandleStopFireTimer))
  (|CallParentFunction))

(event EventUseAmmo
  ;[1 1 1] Override use ammo function from base class
  (|CallParentFunction)
  (Ammo|UseAmmoOverride))

(event EventOnUnequip
  ;[1 1 1] If item is not usable after unequip destroy it
  (|CallParentFunction)
  (if (and (== (CallFunction|GetCurrentAmmo) 0) (not (CallFunction|HasInfiniteAmmo)))
    (Actor|SetLifeSpan 0.5)))

(fn ConstructionScript
  (|CallParentFunction))

(fn HandlFiringOverride
  (bind _mypawn (Variables|Default|GetMyPawn))
  (bind _mypawn_2 (Variables|Default|GetMyPawn))
  (CallFunction|ShowDebugMessage "BaseMelee_BP" "HandleFiring_Override" (Utilities|String|ToString(Name) (Variables|Default|GetWeaponTag)) "NewEnumerator0")
  (Utilities|IsValid _mypawn_2
    (:Is%20Valid
      (if (and (Variables|Default|GetbWantsToFire) (not (Default|IsDying _mypawn_2)))
        (Variables|Internal|SetbIsAmmoUsed false)
        (Utilities|FlowControl|Sequence
          (:then_0
            (if (and (or (> (CallFunction|GetCurrentAmmo) 0) (CallFunction|HasInfiniteAmmo)) (CallFunction|CanFire))
              (Utilities|IsValid (Variables|Default|GetMyPawn)
                (:Is%20Valid
                  (bind _asaicontroller_bp (Utilities|Casting|CastToAIController_BP (Pawn|GetController (Variables|Default|GetMyPawn)))
                    (:then
                      ;[1 1 1] Update attack counter
                      (bind _boutcontinue (Default|UpdateAttackCounter _asaicontroller_bp))
                      (if _boutcontinue
                        ;[1 1 1] Simulate fire only on clients
                        (if (not (Networking|IsDedicatedServer)) :!label _label
                          (CallFunction|SimulateWeaponFire))
                        (else
                          (Default|StopAttack (Variables|Default|GetMyPawn)))))
                    (:CastFailed
                      (goto _label)))))
              (else
                (Default|StopAttack (Variables|Default|GetMyPawn)))))
          (:then_1
            (Utilities|IsValid _mypawn
              (:Is%20Valid
                (if (Pawn|IsLocallyControlled _mypawn)
                  (Utilities|FlowControl|Sequence
                    (:then_0
                      ;[1 1 1] Ask server to handle fire
                      (if (Utilities|Enum|NotEqual(Enum) (Networking|GetLocalRole) "ROLE_Authority")
                        (CallFunction|ServerHandleFiring)))
                    (:then_1
                      ;[1 1 1] Setup refire timer
                      ;;[1 1 1] Check weapon state
                      (if (and (Utilities|Enum|Equal(Enum) (Variables|Default|GetCurrentState) "NewEnumerator1") (> (- (Variables|Default|GetFireAnimationDuration) 0.1) 0.0))
                        ;;[1 1 1] Setup timer for handle firing
                        (bind _returnvalue (Utilities|Time|SetTimerbyFunctionName self "HandleFiring" (- (Variables|Default|GetFireAnimationDuration) 0.1)))
                        (Variables|Default|SetHandleFiringTimer _returnvalue)))
                    (:then_2
                      ;[1 1 1] Auto firing check only for players
                      (if (Utilities|ClassIsChildOf (Utilities|GetClass (Variables|Default|GetMyPawn)) "/Game/UltimateCharacter/Blueprints/Characters/PlayerCharacter_BP.PlayerCharacter_BP_C")
                        (if (not (Variables|Default|GetbAutoFiring))
                          (Variables|Default|SetbWantsToFire false)))))))))
          (:then_2
            ;[1 1 1] Store last fire time
            (Variables|Default|SetLastFireTime (Utilities|Time|GetTimeSeconds) :!label _label_2)))))
    (:Is%20Not%20Valid
      (CallFunction|ShowDebugMessage "BaseMelee_BP" "HandleFiring_Override" "MyPawn is not valid" "NewEnumerator2")
      (goto _label_2))))

(fn InternalFireWeapon
  (CallFunction|ShowDebugMessage "BaseMelee_BP" "InternalFireWeapon" (Utilities|String|ToString(Name) (Variables|Default|GetWeaponTag)) "NewEnumerator0")
  ;[1 1 1] Calculate start and end location for weapon trace
  (LocalVariables|SetTempStartTrace (Weapon|GetDamageStartLocation))
  (LocalVariables|SetTempAim (CallFunction|GetAdjustedAim))
  (bind _output_get (LocalVariables|SetTempEndTrace (+ (LocalVariables|GetTempStartTrace) (* (LocalVariables|GetTempAim) (.TraceDistance (Utilities|Struct|BreakFMeleeInfo (Variables|UltimateCharacter|GetMeleeConfig)))))))
  (bind _outhit (Weapon|WeaponTrace (LocalVariables|GetTempStartTrace) _output_get))
  ;[1 1 1] Process hit location
  (Weapon|ProcessHit _outhit (LocalVariables|GetTempStartTrace) (CallFunction|GetAdjustedAim)))

(fn GetDamageStartLocation
  (Utilities|IsValid (Variables|Default|GetMyPawn)
    (:Is%20Valid
      ;[1 1 1] Get trace start location
      (return (CallFunction|GetStartFireLocation(Muzzle))))
    (:Is%20Not%20Valid
      (CallFunction|ShowDebugMessage "BaseMelee_BP" "GetDamageStartLocation" "Instigator is not valid" "NewEnumerator2")
      (return "0, 0, 0"))))

(fn WeaponTrace
  (params (InStartLocation :type Vector) (InTarget :type Vector))
  (bind _returnvalue (Components|GetOwner))
  (bind _mypawn (Variables|Default|GetMyPawn))
  (bind _meleeconfig (Variables|UltimateCharacter|GetMeleeConfig))
  (bind _bshowdebug (Variables|Default|GetbShowDebug))
  (bind (_buselinetrace _halfsize _orientation) (Utilities|Struct|BreakFMeleeInfo _meleeconfig))
  (bind _array (Utilities|Array|MakeArray _mypawn))
  (bind _returnvalue_2 (select _bshowdebug "Persistent" "None"))
  ;[1 1 1] Doing line or box trace depends on sword config
  (if _buselinetrace
    (bind _outhit (Collision|LineTraceByChannel InStartLocation InTarget "TraceTypeQuery3" false _array _returnvalue_2))
    (LocalVariables|SetTempHitResult _outhit)
    (else
      (bind _outhit_2 (Collision|BoxTraceByChannel InStartLocation InTarget _halfsize _orientation "TraceTypeQuery3" false _array _returnvalue_2))
      (LocalVariables|SetTempHitResult _outhit_2)))
  (if (and (.bBlockingHit (Collision|BreakHitResult (LocalVariables|GetTempHitResult))) (== (.HitActor (Collision|BreakHitResult (LocalVariables|GetTempHitResult))) _returnvalue))
    (CallFunction|ShowDebugMessage "BaseMelee_BP" "WeaponTrace" (Utilities|String|Append (Utilities|GetDisplayName _returnvalue) "  is hitting himself, try to move start fire location (Muzzle Location)") "NewEnumerator3"))
  (return (LocalVariables|GetTempHitResult)))

(fn ProcessHit
  (params (InImpact :type Hit%20Result%20Structure) (InOrigin :type Vector) (InSwordDir :type Vector))
  (bind _hitactor (Collision|BreakHitResult InImpact))
  (bind _mypawn (Variables|Default|GetMyPawn))
  (if (CallFunction|ShouldDealDamage _hitactor)
    (if (Variables|Internal|GetbIsAmmoUsed)
      ;[1 1 1] Deal damage to the target & stop tracing more if hit something
      (bind (_boutblocked _outdamagepercent) (CallFunction|BlockCheck InImpact :!label _label))
      (if _boutblocked
        (LocalVariables|SetTempDamagePercent _outdamagepercent)
        (if (> (LocalVariables|GetTempDamagePercent) 0)
          (CallFunction|DealDamage InImpact InSwordDir (LocalVariables|GetTempDamagePercent) :!label _label_2))
        (else
          (goto _label_2)))
      (if (Utilities|Struct|BreakFMeleeInfo (Variables|UltimateCharacter|GetMeleeConfig))
        _
        (elif (Utilities|ClassIsChildOf (Utilities|GetClass _hitactor) "/Game/UltimateCharacter/Blueprints/Characters/BaseCharacter_BP.BaseCharacter_BP_C")
          (Weapon|ToggleSwordFire false)))
      (Utilities|FlowControl|Sequence :!label _label_3
        (:then_0
          (if (Utilities|Enum|Equal(Enum) (Networking|GetLocalRole) "ROLE_Authority")
            (Variables|Internal|SetHitNotify (Utilities|Struct|MakeFMeleeHitInfo InOrigin))))
        (:then_1))
      (else
        ;[1 1 1] If ammo not used reduce the ammo count only when weapon hit something
        (Utilities|IsValid _mypawn
          (:Is%20Valid
            (if (Pawn|IsLocallyControlled _mypawn)
              (CallFunction|UseAmmo)
              (Variables|Default|SetBurstCounter (+ (Variables|Default|GetBurstCounter) 1))
              (Variables|Internal|SetbIsAmmoUsed true)
              (goto _label))))))
    (else
      (goto _label_3))))

(fn OnRepHitNotify
  (if (Utilities|Enum|Equal(Enum) (Networking|GetLocalRole) "ROLE_Authority")
    (Weapon|SimulateHit (Variables|Internal|GetHitNotify))))

(fn SimulateHit
  (params (InHit :type F%20Melee%20Hit%20Info%20Structure))
  ;[1 1 1] TODO : Different from weapon instant
  (LocalVariables|SetStartTrace (Weapon|GetDamageStartLocation))
  (bind _output_get (LocalVariables|SetEndTrace (+ (.origin InHit) (* (CallFunction|GetAdjustedAim) (.TraceDistance (Utilities|Struct|BreakFMeleeInfo (Variables|UltimateCharacter|GetMeleeConfig)))))))
  (bind _outhit (Weapon|WeaponTrace (LocalVariables|GetStartTrace) _output_get))
  (bind _output_get_2 (LocalVariables|SetImpact _outhit))
  ;[1 1 1] TODO: Spawn impact effect
  (if (.bBlockingHit (Collision|BreakHitResult _output_get_2))
    _))

(fn OnBurstStartedOverride
  (bind _fireanimationduration (Variables|Default|GetFireAnimationDuration))
  (CallFunction|ShowDebugMessage "BaseMelee_BP" "OnBurstedStarted_Override" (Utilities|String|ToString(Name) (Variables|Default|GetWeaponTag)) "NewEnumerator0")
  (if (Math|Boolean|ANDBoolean (> (Variables|Default|GetLastFireTime) 0.0) (> _fireanimationduration 0.0) (> (+ _fireanimationduration (Variables|Default|GetLastFireTime)) (Utilities|Time|GetTimeSeconds)))
    ;[1 1 1] Check and execute combo for player
    (if (not (Utilities|ClassIsChildOf (Utilities|GetClass (Variables|Default|GetMyPawn)) "/Game/UltimateCharacter/Blueprints/Characters/PlayerCharacter_BP.PlayerCharacter_BP_C"))
      ;[1 1 1] Handle refiring timer
      (bind _returnvalue (Utilities|Time|SetTimerbyFunctionName self "HandleFiring" (- (+ (Variables|Default|GetLastFireTime) (Variables|Default|GetFireAnimationDuration)) (Utilities|Time|GetTimeSeconds)) :!label _label))
      (Variables|Default|SetHandleFiringTimer _returnvalue)
      (elif (Default|IsComboActive (Variables|Default|GetMyPawn))
        (Utilities|Time|ClearandInvalidateTimerbyHandle (Variables|Internal|GetHandleStopFireTimer))
        (Utilities|Time|ClearandInvalidateTimerbyHandle (Variables|Default|GetHandleFiringTimer))
        (CallFunction|HandleFiring)
        (else
          (goto _label))))
    (else
      (CallFunction|HandleFiring))))

(fn ToggleSwordFire
  (params (InToggle :type Boolean))
  (CallFunction|ShowDebugMessage "BaseMelee_BP" "ToggleSwordFire" (Utilities|String|ToString(Name) (Variables|Default|GetWeaponTag)) "NewEnumerator0")
  (if (Utilities|Enum|Equal(Enum) (Variables|Default|GetCurrentState) "NewEnumerator1")
    (Variables|Internal|SetFireSword InToggle)
    (else
      (Variables|Internal|SetFireSword false)))
  (return (Variables|Internal|GetFireSword)))

(fn GetDamageInfo
  (bind _meleeconfig (Variables|UltimateCharacter|GetMeleeConfig))
  (bind (_hitdamage _damagetype) (Utilities|Struct|BreakFMeleeInfo _meleeconfig))
  (return _hitdamage _damagetype))

(fn InitializeCombo
  (params (InComboe :type Map%20of%20Names%20to%20Reals))
  ;[1 1 1] Store combo info
  (Variables|Default|SetComboSections InComboe))

(fn StopFireOverride
  (bind _handlefiringtimer (Variables|Default|GetHandleFiringTimer))
  (bind _returnvalue (Utilities|Time|GetTimerRemainingTimebyHandle _handlefiringtimer))
  (CallFunction|ShowDebugMessage "BaseMelee_BP" "StopFire" (Utilities|String|ToString(Name) (Variables|Default|GetWeaponTag)) "NewEnumerator0")
  (if (Utilities|Enum|NotEqual(Enum) (Networking|GetLocalRole) "ROLE_Authority")
    ;[1 1 1] Add delay to player stop fire to prevent stop tracing before ending the animation
    (CallFunction|ServerStopFire))
  (if (> _returnvalue 0.1)
    (bind _returnvalue_2 (Utilities|Time|SetTimerbyFunctionName self "StopFire" (- _returnvalue 0.05)))
    (Variables|Internal|SetHandleStopFireTimer _returnvalue_2)
    (else
      (Variables|Default|SetbWantsToFire false)
      (Utilities|Time|ClearandInvalidateTimerbyHandle (Variables|Default|GetHandleFiringTimer))
      (CallFunction|DetermineWeaponState)
      (Ammo|OutOfUseCheck))))

(fn InitializeAmmo
  (CallFunction|ShowDebugMessage "BaseMelee_BP" "InitializeAmmo" (Utilities|String|ToString(Name) (Variables|Default|GetWeaponTag)) "NewEnumerator0")
  (Variables|Default|SetCurrentAmmo (Utilities|Struct|BreakFMeleeInfo (Variables|UltimateCharacter|GetMeleeConfig)))
  (return true))

(fn UseAmmoOverride
  (CallFunction|ShowDebugMessage "BaseMelee_BP" "UseAmmo_Override" (Utilities|String|ToString(Name) (Variables|Default|GetWeaponTag)) "NewEnumerator0")
  (if (not (CallFunction|HasInfiniteAmmo))
    ;[1 1 1] Use ammo
    (Variables|Default|SetCurrentAmmo (- (Variables|Default|GetCurrentAmmo) 1))))

(fn GetMaxAmmo
  (return (Utilities|Struct|BreakFMeleeInfo (Variables|UltimateCharacter|GetMeleeConfig))))

(fn OutOfUseCheck
  (bind _mypawn (Variables|Default|GetMyPawn))
  (CallFunction|ShowDebugMessage "BaseMelee_BP" "OutOfUseCheck" (Utilities|String|ToString(Name) (Variables|Default|GetWeaponTag)) "NewEnumerator0")
  ;[1 1 1] Try to remove from pawn if weapon is not usable
  (if (and (< (CallFunction|GetCurrentAmmo) 1) (not (CallFunction|HasInfiniteAmmo)))
    (Utilities|IsValid _mypawn
      (:Is%20Valid
        (Default|RemoveWeapon _mypawn self false)))))

(fn HasInfiniteAmmo
  (return (Utilities|Struct|BreakFMeleeInfo (Variables|UltimateCharacter|GetMeleeConfig))))