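; Hitscan gun weapon that fires line traces within a spread cone that widens per shot and resets after each burst.
; The locally controlled client reports hits and misses to the server, which checks hits against view direction and a bounds-based leeway.
; Confirmed hits apply block-adjusted damage and spawn trail and impact effects.
; Replicated HitNotify carries the random seed and spread so non-authority clients re-trace shots for effects.
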(event Custom|ServerNotifyHit
  (params (InImpact :type Hit%20Result%20Structure) (InShootDir :type Vector%20Net%20Quantize%20Normal%20Structure) (InRandomSeed :type Integer) (InReticleSpread :type Float%20%28double-precision%29))
  (bind (_bblockinghit _binitialoverlap _time _distance _location _impactpoint _normal _impactnormal _physmat _hitactor) (Collision|BreakHitResult InImpact))
  (bind (_bblockinghit_2 _binitialoverlap_2 _time_2 _distance_2 _location_2 _impactpoint_2 _normal_2 _impactnormal_2 _physmat_2 _hitactor_2) (Collision|BreakHitResult InImpact))
  (bind _clientsidehitleeway (Variables|Internal|GetClientSideHitLeeway))
  (bind _boxextent (Collision|GetActorBounds _hitactor_2 false false))
  (bind (_x _y _z) (Math|Vector|BreakVector _location_2))
  (bind _rootcomponent (Variables|/Script/Engine.Actor|GetRootComponent _hitactor_2))
  (bind _returnvalue (* _boxextent _clientsidehitleeway))
  (bind _mobility (Variables|/Script/Engine.SceneComponent|GetMobility _rootcomponent))
  (bind (_x_2 _y_2 _z_2) (Math|Vector|BreakVector _returnvalue))
  (Variables|Internal|SetWeaponAngleDot (Math|Float|Absolute(Float) (Math|Trig|Sin(Radians) (/ (* (Math|Trig|GetPI) InReticleSpread) 1.8e+02))))
  (Utilities|IsValid (Game|GetInstigator)
    (:Is%20Valid
      (Utilities|IsValid _hitactor
        (:Is%20Valid
          (bind _output_get (Variables|Internal|SetViewDir (Math|Vector|Normalize (- _location (CallFunction|GetStartFireLocation(Muzzle)))) :!label _label))
          (bind _output_get_2 (Variables|Internal|SetViewDotHitDir (Math|Vector|DotProduct (Math|Rotator|GetRotationXVector (Pawn|GetControlRotation (Game|GetInstigator) :!class /Script/Engine.Pawn)) _output_get)))
          (if (> _output_get_2 (- (Variables|Internal|GetAllowedViewDotHitDir) (Variables|Internal|GetWeaponAngleDot)))
            (if (Utilities|Enum|NotEqual(Enum) (Variables|Default|GetCurrentState) "NewEnumerator0")
              (if (== _hitactor_2 0)
                (if _bblockinghit_2
                  (Weapon|ProcessInstantHitConfirmed InImpact (CallFunction|GetStartFireLocation(Muzzle)) InShootDir InRandomSeed InReticleSpread :!label _label_2))
                (elif (or (Utilities|Enum|Equal(Enum) _mobility "Static") (Utilities|Enum|Equal(Enum) _mobility "Stationary"))
                  (goto _label_2)
                  (else
                    (bind _output_get_3 (Variables|Internal|SetBoxExtent (Math|Vector|MakeVector (Math|Float|Max(Float) 2e+01 _x_2) (Math|Float|Max(Float) 2e+01 _y_2) (Math|Float|Max(Float) 2e+01 _z_2))))
                    (if (Math|Boolean|ANDBoolean (< (Math|Float|Absolute(Float) (- _x (.X (Math|Vector|BreakVector _output_get_3)))) (.X (Math|Vector|BreakVector _output_get_3))) (< (Math|Float|Absolute(Float) (- _y (.Y (Math|Vector|BreakVector _output_get_3)))) (.Y (Math|Vector|BreakVector _output_get_3))) (< (Math|Float|Absolute(Float) (- _z (.Z (Math|Vector|BreakVector _output_get_3)))) (.Z (Math|Vector|BreakVector _output_get_3))))
                      (goto _label_2))))))))
        (:Is%20Not%20Valid
          (if _bblockinghit
            (goto _label)))))))

(event Custom|ServerNotifyMiss
  (params (InShootDir :type Vector%20Net%20Quantize%20Normal%20Structure) (InRandomSeed :type Integer) (InReticleSpread :type Float%20%28double-precision%29))
  (Variables|Internal|SetHitNotify (Utilities|Struct|MakeFInstantHitInfo (CallFunction|GetStartFireLocation(Muzzle)) InReticleSpread InRandomSeed))
  ;[1 1 1] Play FX Localy
  (if (Networking|IsDedicatedServer)
    (Effects|SpawnTrailEffect (* (+ (CallFunction|GetStartFireLocation(Muzzle)) InShootDir) (Utilities|Struct|BreakFInstantWeaponData (Variables|UltimateCharacter|GetInstantGunConfig))))))

(event EventBeginPlay
  (|CallParentFunction)
  (Variables|Default|SetWeaponType "NewEnumerator1"))

(event Collision|EventActorBeginOverlap
  (params (OtherActor :type Actor%20Object%20Reference))
  (|CallParentFunction OtherActor) ; This node is disabled and will not be called.\nDrag off pins to build functionality.
)

(event EventTick
  (params (DeltaSeconds :type Float%20%28single-precision%29))
  (|CallParentFunction DeltaSeconds) ; This node is disabled and will not be called.\nDrag off pins to build functionality.
)

(event EventFireWeapon
  ;[1 1 1] Override fire weapon
  (Weapon|InternalFireWeapon))

(event EventOnBurstFinished
  ;[1 1 1] Override burst function to reset firing spread
  (|CallParentFunction)
  (Variables|Internal|SetCurrentFiringSpread 0.0))

(fn ConstructionScript
  (|CallParentFunction))

(fn GetCurrentSpread
  (bind _mypawn (Variables|Default|GetMyPawn))
  ;[1 1 1] Calculate bullets spread
  (LocalVariables|SetTempSpread (+ (Variables|Internal|GetCurrentFiringSpread) (Utilities|Struct|BreakFInstantWeaponData (Variables|UltimateCharacter|GetInstantGunConfig))))
  (Utilities|IsValid _mypawn
    (:Is%20Valid
      (if (Default|IsTargeting _mypawn)
        (return (* (LocalVariables|GetTempSpread) (Utilities|Struct|BreakFInstantWeaponData (Variables|UltimateCharacter|GetInstantGunConfig))))
        (else
          _)))
    (:Is%20Not%20Valid
      _))
  (return (LocalVariables|GetTempSpread)))

(fn GetAmmoType
  (return "NewEnumerator0"))

(fn OnRepHitNotify
  (bind _hitnotify (Variables|Internal|GetHitNotify))
  (if (not (Utilities|Enum|Equal(Enum) (Networking|GetLocalRole) "ROLE_Authority"))
    (Weapon|SimulateInstantHit (.origin _hitnotify) (.randomseed _hitnotify) (.reticlespread _hitnotify))))

(fn SimulateInstantHit
  (params (InOrigin :type Vector) (InRandomSeed :type Integer) (ReticleSpread :type Float%20%28double-precision%29))
  (CallFunction|ShowDebugMessage "GunInstant_BP" "SimulateInstantHit" (Utilities|String|ToString(Name) (Variables|Default|GetWeaponTag)) "NewEnumerator0")
  (Math|Random|SetRandomStreamSeed (LocalVariables|GetWeaponRandomStream) InRandomSeed)
  (LocalVariables|SetConeHalfAngle (Math|Trig|DegreesToRadians (* ReticleSpread 0.5)))
  ;[1 1 1] Start weapon trace from aimig direction of camera to the end point of weapon range
  (bind _output_get (LocalVariables|SetAimDir (CallFunction|GetAdjustedAim)))
  (LocalVariables|SetShootDir (Class|KismetMathLibrary|RandomUnitVectorinConeinRadiansfromStream (LocalVariables|GetWeaponRandomStream) _output_get (LocalVariables|GetConeHalfAngle)))
  (bind _output_get_2 (LocalVariables|SetEndTrace (+ InOrigin (* (LocalVariables|GetShootDir) (Utilities|Struct|BreakFInstantWeaponData (Variables|UltimateCharacter|GetInstantGunConfig))))))
  (bind _outhit (CallFunction|WeaponTrace InOrigin _output_get_2))
  (bind _output_get_3 (LocalVariables|SetImpact _outhit))
  ;[1 1 1] Spawn effects
  (if (.bBlockingHit (Collision|BreakHitResult _output_get_3))
    (Effects|SpawnImpactEffect (LocalVariables|GetImpact))
    (else
      (Effects|SpawnTrailEffect (LocalVariables|GetEndTrace)))))

(fn ProcessInstantHitConfirmed
  (params (InImpact :type Hit%20Result%20Structure) (InOrigin :type Vector) (InShootDir :type Vector) (InRandomSeed :type Integer) (InReticleSpread :type Float%20%28double-precision%29))
  (CallFunction|ShowDebugMessage "GunInstant_BP" "ProcessInstantHitConfirmed" (Utilities|String|ToString(Name) (Variables|Default|GetWeaponTag)) "NewEnumerator0")
  (if (CallFunction|ShouldDealDamage (.HitActor (Collision|BreakHitResult InImpact)))
    ;[1 1 1] Check if target can block attack
    (bind (_boutblocked _outdamagepercent) (CallFunction|BlockCheck InImpact))
    (if _boutblocked
      (LocalVariables|SetTempDamagePercent _outdamagepercent)
      (if (> (LocalVariables|GetTempDamagePercent) 0)
        ;[1 1 1] Deal damage to the hited actor
        (CallFunction|DealDamage InImpact InShootDir (LocalVariables|GetTempDamagePercent) :!label _label))
      (else
        (goto _label))))
  (Utilities|FlowControl|Sequence
    (:then_0
      (if (Utilities|Enum|Equal(Enum) (Networking|GetLocalRole) "ROLE_Authority")
        (Variables|Internal|SetHitNotify (Utilities|Struct|MakeFInstantHitInfo InOrigin InReticleSpread InRandomSeed))))
    (:then_1
      ;[1 1 1] Spawn weapon effects
      (if (not (Networking|IsDedicatedServer))
        (Effects|SpawnTrailEffect (+ InOrigin (* InShootDir (Utilities|Struct|BreakFInstantWeaponData (Variables|UltimateCharacter|GetInstantGunConfig)))))
        (Effects|SpawnImpactEffect InImpact)))))

(fn SpawnTrailEffect
  (params (InEndPoint :type Vector))
  (CallFunction|ShowDebugMessage "GunInstant_BP" "SpawnImpactEffect" (Utilities|String|ToString(Name) (Variables|Default|GetWeaponTag)) "NewEnumerator0")
  (Utilities|IsValid (Variables|UltimateCharacter|GetTrailFX)
    (:Is%20Valid
      (bind _returnvalue (Effects|SpawnEmitteratLocation (Variables|UltimateCharacter|GetTrailFX) (CallFunction|GetStartFireLocation(Muzzle))))
      (Utilities|IsValid _returnvalue
        (:Is%20Valid
          (Effects|Components|ParticleSystem|SetVectorParameter _returnvalue (Variables|UltimateCharacter|GetTrailTargetParam) InEndPoint))))))

(fn ProcessInstantHit
  (params (InImpact :type Hit%20Result%20Structure) (InOrigin :type Vector) (InShootDir :type Vector) (InRandomSeed :type Integer) (InReticleSpread :type Float%20%28double-precision%29))
  (bind _mypawn (Variables|Default|GetMyPawn))
  (bind _returnvalue (Math|Vector|MakeVectorNetQuantizeNormal (.x InShootDir) (.y InShootDir) (.z InShootDir)))
  (bind (_bblockinghit _binitialoverlap _time _distance _location _impactpoint _normal _impactnormal _physmat _hitactor) (Collision|BreakHitResult InImpact))
  (CallFunction|ShowDebugMessage "GunInstant_BP" "ProcessInstantHit" (Utilities|String|ToString(Name) (Variables|Default|GetWeaponTag)) "NewEnumerator0")
  (Utilities|IsValid _mypawn
    (:Is%20Valid
      (if (Math|Boolean|ANDBoolean (Pawn|IsLocallyControlled _mypawn) (Math|Boolean|Equal(Boolean) (Networking|IsDedicatedServer) false) (Math|Boolean|Equal(Boolean) (Class|KismetSystemLibrary|IsStandalone) false))
        (Utilities|IsValid _hitactor
          (:Is%20Valid
            (if (Utilities|Enum|Equal(Enum) (Class|Actor|GetRemoteRole _hitactor) "ROLE_Authority")
              (CallFunction|ServerNotifyHit InImpact _returnvalue InRandomSeed InReticleSpread :!label _label)))
          (:Is%20Not%20Valid
            (if (== _hitactor 0)
              (if _bblockinghit
                (goto _label)
                (else
                  (CallFunction|ServerNotifyMiss _returnvalue InRandomSeed InReticleSpread))))))))
    (:Is%20Not%20Valid
      _))
  (Weapon|ProcessInstantHitConfirmed InImpact InOrigin InShootDir InRandomSeed InReticleSpread))

(fn SpawnImpactEffect
  (params (InImpact :type Hit%20Result%20Structure))
  (bind (_bblockinghit _binitialoverlap _time _distance _location _impactpoint _normal _impactnormal _physmat _hitactor _hitcomponent) (Collision|BreakHitResult InImpact))
  (bind _returnvalue (* _impactnormal 1e+01))
  (CallFunction|ShowDebugMessage "GunInstant_BP" "SpawnImpactEffect" (Utilities|String|ToString(Name) (Variables|Default|GetWeaponTag)) "NewEnumerator0")
  (LocalVariables|SetUseImpact InImpact)
  (if (and _bblockinghit (!= (Variables|UltimateCharacter|GetImpactEffect) 0))
    (Utilities|FlowControl|Sequence
      (:then_0
        (Utilities|IsValid _hitcomponent
          (:Is%20Not%20Valid
            (LocalVariables|SetStartTrace (+ _impactpoint _returnvalue))
            (LocalVariables|SetEndTrace (- _impactpoint _returnvalue))
            (bind _outhit (CallFunction|WeaponTrace (LocalVariables|GetStartTrace) (LocalVariables|GetEndTrace)))
            (LocalVariables|SetUseImpact _outhit))))
      (:then_1
        (LocalVariables|SetSpawnTransform (Math|Transform|MakeTransform _impactpoint (Math|Conversions|RotationFromXVector _normal))))
      (:then_2
        ;[1 1 1] Spawn impact effect
        (bind _returnvalue_2 (Game|SpawnActorfromClass (Variables|UltimateCharacter|GetImpactEffect) (LocalVariables|GetSpawnTransform) "Undefined" "SelectDefaultAtRuntime" 0 0))
        (Variables|/Game/UltimateCharacter/Blueprints/Effects/ImpactEffects/ImpactEffect_BP.ImpactEffect_BP_C|SetSurfaceHit _returnvalue_2 (LocalVariables|GetUseImpact))))))

(fn InternalFireWeapon
  (bind _instantgunconfig (Variables|UltimateCharacter|GetInstantGunConfig))
  (bind (_firingspreadincrement _firingspreadmax) (Utilities|Struct|BreakFInstantWeaponData _instantgunconfig))
  (CallFunction|ShowDebugMessage "GunInstant_BP" "InternalFireWeapon" (Utilities|String|ToString(Name) (Variables|Default|GetWeaponTag)) "NewEnumerator0")
  (bind _output_get (LocalVariables|SetRandomSeed (Math|Random|RandomInteger -1)))
  (Math|Random|SetRandomStreamSeed (LocalVariables|GetWeaponRandomStream) _output_get)
  (LocalVariables|SetCurrentSpread (Weapon|GetCurrentSpread))
  (LocalVariables|SetConeHalfAngle (Math|Trig|DegreesToRadians (* (Variables|Internal|GetCurrentFiringSpread) 0.5)))
  ;[1 1 1] Get the aim & fire start location
  (bind _output_get_2 (LocalVariables|SetAimDir (CallFunction|GetAdjustedAim)))
  (LocalVariables|SetStartTrace (CallFunction|GetCameraDamageStartLocation _output_get_2))
  (LocalVariables|SetShootDir (Class|KismetMathLibrary|RandomUnitVectorinConeinRadiansfromStream (LocalVariables|GetWeaponRandomStream) (LocalVariables|GetAimDir) (LocalVariables|GetConeHalfAngle)))
  (LocalVariables|SetEndTrace (+ (LocalVariables|GetStartTrace) (* (LocalVariables|GetShootDir) (Utilities|Struct|BreakFInstantWeaponData (Variables|UltimateCharacter|GetInstantGunConfig)))))
  ;[1 1 1] Start weapon trace and process the result
  (bind _outhit (CallFunction|WeaponTrace (LocalVariables|GetStartTrace) (LocalVariables|GetEndTrace)))
  (Weapon|ProcessInstantHit _outhit (LocalVariables|GetStartTrace) (LocalVariables|GetShootDir) (LocalVariables|GetRandomSeed) (LocalVariables|GetCurrentSpread))
  (Variables|Internal|SetCurrentFiringSpread (Math|Float|Min(Float) _firingspreadmax (+ (Variables|Internal|GetCurrentFiringSpread) _firingspreadincrement))))

(fn GetDamageInfo
  (bind _instantgunconfig (Variables|UltimateCharacter|GetInstantGunConfig))
  (bind (_hitdamage _damagetype) (Utilities|Struct|BreakFInstantWeaponData _instantgunconfig))
  (return (Math|Conversions|ToFloat(Integer) _hitdamage) _damagetype))