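; Base bow weapon that cannot be equipped alongside other items and fires arrow projectiles.
; While bending is active, a draw value builds on Tick up to a maximum, scaling trace and arrow distance.
; Firing traces along the adjusted camera aim for a target, then calls ServerFireProjectile to spawn and launch the arrow from the muzzle.
; Ammo reads as one when the pawn's current item is an arrow, otherwise zero.
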(event EventBeginPlay
  (|CallParentFunction)
  ;[1 1 1] We can't equip bow with other weapons/items!
  (Variables|Default|SetbEquipWithOthers false))

(event Collision|EventActorBeginOverlap
  (params (OtherActor :type Actor%20Object%20Reference))
  (|CallParentFunction OtherActor) ; This node is disabled and will not be called.\nDrag off pins to build functionality.
)

(event EventTick
  (params (DeltaSeconds :type Float%20%28single-precision%29))
  (|CallParentFunction DeltaSeconds)
  (CallFunction|UpdateBending DeltaSeconds))

(event EventUpdateUIAmmo
  ;[1 1 1] Override ammo count on UI
  (UI|UpdateUIAmmoOverride))

(event EventServerFireProjectile
  (params (InOrigin :type Vector :default "0, 0, 0") (InShootDir :type Rotator :default "0, 0, 0"))
  (CallFunction|ShowDebugMessage "BaseBow_BP" "ServerFireProjectile" "" "NewEnumerator0")
  (bind _returnvalue (Game|SpawnActorfromClass (Variables|Default|GetProjectileClass) (Math|Transform|MakeTransform InOrigin InShootDir) "Undefined" "SelectDefaultAtRuntime" self (Variables|Default|GetInstigator)))
  (Utilities|IsValid _returnvalue
    (:Is%20Valid
      (bind _asbase_arrow_projectile_bp (Utilities|Casting|CastToBase_Arrow_ProjectileBP _returnvalue))
      (Default|FireArrow _asbase_arrow_projectile_bp (Math|Float|MapRangeClamped (Bow|GetBendingAmount) 0.0 (Variables|UltimateCharacter|GetMaxBending) 256.0 (Variables|UltimateCharacter|GetMaxDistance)) (Variables|Internal|GetTargetLocation)))))

(event EventInternalFireWeapon
  (Weapon|InternalFireWeaponOverride))

(fn ConstructionScript
  (|CallParentFunction))

(fn GetBendingAmount
  (return (Math|Float|MapRangeClamped (Variables|Internal|GetCurrentBending) 0.0 (Variables|UltimateCharacter|GetMaxBending) 0.0 1.0)))

(fn DrawArrow
  (params (InMontage :type F%20Weapon%20Animation%20Structure))
  (CallFunction|ShowDebugMessage "BaseBow_BP" "DrawArrow" "" "NewEnumerator0")
  (CallFunction|PlayWeaponAnimation InMontage))

(fn UpdateUIAmmoOverride
  (bind _mypawn (Variables|Default|GetMyPawn))
  (Utilities|IsValid _mypawn
    (:Is%20Valid
      (CallFunction|ShowDebugMessage "BaseBow_BP" "UpdateUIAmmoOverride" "" "NewEnumerator0")
      (Default|UpdateUIAmmo _mypawn (Variables|Default|GetWeaponTag) (CallFunction|GetCurrentAmmo) -1))))

(fn SetArrowTag
  (params (InTag :type Name))
  (CallFunction|ShowDebugMessage "BaseBow_BP" "SetArrowTag" "" "NewEnumerator0")
  (Variables|Internal|SetArrowTag InTag))

(fn GetArrowTag
  (return (Variables|Internal|GetArrowTag)))

(fn SetBending
  (params (bInBending :type Boolean))
  (Variables|Internal|SetbBending bInBending))

(fn UpdateBending
  (params (InDeltaTime :type Float%20%28double-precision%29))
  (if (Variables|Internal|GetbBending)
    (Variables|Internal|SetCurrentBending (Math|Float|Clamp(Float) (+ (Variables|Internal|GetCurrentBending) (* InDeltaTime (Variables|UltimateCharacter|GetBendingMultiplier))) 0.0 (Variables|UltimateCharacter|GetMaxBending)))
    (else
      (Variables|Internal|SetCurrentBending 0.0))))

(fn GetCurrentAmmo
  (bind _mypawn (Variables|Default|GetMyPawn))
  (bind _currentitem (Variables|/Game/UltimateCharacter/Blueprints/Characters/BaseCharacter_BP.BaseCharacter_BP_C|GetCurrentItem _mypawn))
  (Utilities|IsValid _currentitem
    (:Is%20Valid
      (if (Utilities|ClassIsChildOf (Utilities|GetClass _currentitem) "/Game/UltimateCharacter/Blueprints/Items/Arrow/Base_Arrow_ItemBP.Base_Arrow_ItemBP_C")
        (return 1)
        (else
          _)))
    (:Is%20Not%20Valid
      _))
  (return 0))

(fn GetCurrentAmmoinClip
  (return (CallFunction|GetCurrentAmmo)))

(fn InternalFireWeaponOverride
  (CallFunction|ShowDebugMessage "BaseBow_BP" "InternalFireWeapon_Override" (Utilities|String|ToString(Name) (Variables|Default|GetWeaponTag)) "NewEnumerator0")
  (bind _output_get (LocalVariables|SetRandomSeed (Math|Random|RandomInteger -1)))
  (Math|Random|SetRandomStreamSeed (LocalVariables|GetWeaponRandomStream) _output_get)
  (bind _output_get_2 (LocalVariables|SetAimDir (CallFunction|GetAdjustedAim)))
  (LocalVariables|SetStartTrace (CallFunction|GetCameraDamageStartLocation _output_get_2))
  (LocalVariables|SetEndTrace (+ (LocalVariables|GetStartTrace) (* (LocalVariables|GetAimDir) (Math|Float|MapRangeClamped (Bow|GetBendingAmount) 0.0 (Variables|UltimateCharacter|GetMaxBending) 256.0 (Variables|UltimateCharacter|GetMaxDistance)))))
  (bind _outhit (CallFunction|WeaponTrace (LocalVariables|GetStartTrace) (LocalVariables|GetEndTrace)))
  (if (.bBlockingHit (Collision|BreakHitResult _outhit))
    (Variables|Internal|SetTargetLocation (.ImpactPoint (Collision|BreakHitResult _outhit)))
    (else
      (Variables|Internal|SetTargetLocation (LocalVariables|GetEndTrace))))
  (CallFunction|ServerFireProjectile (CallFunction|GetStartFireLocation(Muzzle)) (Math|Conversions|RotationFromXVector (LocalVariables|GetAimDir))))