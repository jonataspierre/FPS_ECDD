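; Base bombard actor for area attacks, optionally placed at its instigator, near an AI's target or at the player cursor.
; A timeline-grown sphere deals direct damage on overlap, then destroys the actor; otherwise a looping timer or fixed-size sphere triggers radial damage.
; Damage requires a living instigator, scales with difficulty and can add knockback.
; Targets can block: direct hits use the block's damage percent, while radial hits ignore blockers found by distance and line-trace checks.
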(event OnComponentBeginOverlap(Sphere)
  (params (OverlappedComponent :type Primitive%20Component%20Object%20Reference) (OtherActor :type Actor%20Object%20Reference) (OtherComp :type Primitive%20Component%20Object%20Reference) (OtherBodyIndex :type Integer) (bFromSweep :type Boolean) (SweepResult :type Hit%20Result%20Structure%20%28by%20ref%29))
  (bind _returnvalue (Game|GetInstigator))
  ;[1 1 1] Collision has overlap on an actor
  (if (Math|Boolean|ANDBoolean (!= OtherActor self) (!= _returnvalue (Components|GetOwner OtherActor)) (!= OtherActor _returnvalue) (not (Utilities|Array|ContainsItem (Variables|Internal|GetOverlappingActors) OtherActor)))
    (Utilities|Array|AddUnique (Variables|Internal|GetOverlappingActors) OtherActor)
    (Attack|DoAttack OtherActor)))

(event OnComponentEndOverlap(Sphere)
  (params (OverlappedComponent :type Primitive%20Component%20Object%20Reference) (OtherActor :type Actor%20Object%20Reference) (OtherComp :type Primitive%20Component%20Object%20Reference) (OtherBodyIndex :type Integer))
  ;[1 1 1] Actor end ovelap and remove from damaged actor, if he overlap again will take damage
  (bind _returnvalue (Utilities|Array|RemoveItem (Variables|Internal|GetOverlappingActors) OtherActor))
  (Debug|ShowDebugMessage "BaseBombard_BP" "ShpereEndOverlap" (Utilities|String|Append (Utilities|GetDisplayName OtherActor) (Utilities|String|SelectString " removed " " not removed " _returnvalue) " from damaged actors") "NewEnumerator0"))

(event Custom|AnimateCollision
  ;[1 1 1] Animate collision radius
  (bind _alpha (Timeline|SphereAnimation PlayFromStart)
    (:Update
      (Components|Sphere|SetSphereRadius (Variables|Default|GetSphere) (Math|Float|Lerp (Variables|UltimateCharacter|GetInitialCollisionSize) (Variables|UltimateCharacter|GetMaxDamageRadius) _alpha) true))
    (:Finished
      ;;[1 1 1] Only destroy actor after finishing attack in case of intrrupted by animation or AI
      (Disable|BeforeDisableBombard)
      (Utilities|Time|ClearandInvalidateTimerbyHandle (Variables|Internal|GetAttackTimer))
      (Debug|ShowDebugMessage "BaseBombard_BP" "AnimateCollision" (Utilities|String|Append "Animating collision is finished and destroy attack" (Utilities|String|ToString(Name) (Variables|UltimateCharacter|GetItemTag))) "NewEnumerator0")
      (Actor|DestroyActor))))

(event EventBeginPlay
  ;[1 1 1] Enable bombard after spawn class
  (Enable|EnableBombard)
  (Variables|Internal|SetGameDifficulty (CallFunction|GetGameDifficulty)))

(fn ConstructionScript)

(fn DisableBombard
  ;[1 1 1] Disable and clear timer
  (if (Variables|UltimateCharacter|GetbAnimateCollision)
    (Transformation|DetachFromActor "KeepWorld" "KeepWorld" "KeepWorld")
    (Debug|ShowDebugMessage "BaseBombard_BP" "DisableBombard" "Detach bombard from character" "NewEnumerator0")
    (else
      (Disable|BeforeDisableBombard)
      (Utilities|Time|ClearandInvalidateTimerbyHandle (Variables|Internal|GetAttackTimer))
      (Debug|ShowDebugMessage "BaseBombard_BP" "DisableBombard" "Bombard destroyed" "NewEnumerator0")
      (Actor|DestroyActor))))

(fn DoAttack
  (params (InTarget :type Actor%20Object%20Reference))
  (Debug|ShowDebugMessage "BaseBombard_BP" "DoAttack" (Utilities|String|Append "Apply attack to : " (Utilities|GetDisplayName InTarget)) "NewEnumerator0")
  (Attack|CalculateDamage InTarget)
  (return))

(fn BeforeDisableBombard
  (Debug|ShowDebugMessage "BaseBombard_BP" "Before disable bombard" (Utilities|String|ToString(Name) (Variables|UltimateCharacter|GetItemTag)) "NewEnumerator0"))

(fn EnableBombard
  ;[1 1 1] Setup some initial variables
  (Enable|BeforeEnableBombard)
  (Debug|ShowDebugMessage "BaseBombard_BP" "EnableBombard" (Utilities|String|ToString(Name) (Variables|UltimateCharacter|GetItemTag)) "NewEnumerator0")
  ;[1 1 1] Start animation collision
  (if (Variables|UltimateCharacter|GetbAnimateCollision)
    (CallFunction|AnimateCollision))
  ;[1 1 1] Start auto attack timer
  (if (> (Variables|Internal|GetAutoAttackTimeInterval) 0.0)
    (bind _returnvalue (Utilities|Time|SetTimerbyFunctionName self "DoAutoAttack" (Variables|Internal|GetAutoAttackTimeInterval) true))
    (Variables|Internal|SetAttackTimer _returnvalue)
    (elif (not (Variables|UltimateCharacter|GetbAnimateCollision))
      (Debug|ShowDebugMessage "BaseBombard_BP" "EnableBombard" (Utilities|String|Append "Attack interval is less than zero & Animate collision is disable, Sphere radius for attack manually sets to " (Utilities|String|ToString(Float) (Variables|UltimateCharacter|GetMaxDamageRadius)) " and overlapping actors will get damage") "NewEnumerator0")
      (Components|Sphere|SetSphereRadius (Variables|Default|GetSphere) (Variables|UltimateCharacter|GetMaxDamageRadius) true))))

(fn BeforeEnableBombard
  (Debug|ShowDebugMessage "BaseBombard_BP" "Before enable bombard" (Utilities|String|ToString(Name) (Variables|UltimateCharacter|GetItemTag)) "NewEnumerator0")
  ;[1 1 1] Setup timeline variables
  (Components|Timeline|SetPlayRate (Variables|Default|GetSphereAnimation) (Variables|UltimateCharacter|GetCollisionAnimateRate))
  (Class|TimelineComponent|SetFloatCurve (Variables|Default|GetSphereAnimation) (Variables|UltimateCharacter|GetAnimateCurve) "Alpha")
  ;[1 1 1] Add instigator to this array to ignore apply damage on him self
  (Utilities|Array|AddUnique (Variables|Internal|GetOverlappingActors) (Game|GetInstigator))
  ;[1 1 1] Get and set spawn location
  (if (Variables|UltimateCharacter|GetbSpawnAtTargetLocation)
    (Variables|Internal|SetTargetLocation (Attack|FindAttackLocation))
    (Transformation|SetActorLocation (Variables|Internal|GetTargetLocation) false true)))

(fn CalculateDamage
  (params (InTarget :type Actor%20Object%20Reference))
  (bind _returnvalue (Game|GetInstigator))
  ;[1 1 1] Apply damage to the area under some conditions
  (Utilities|IsValid _returnvalue
    (:Is%20Valid
      (bind _asbase_character_bp (Utilities|Casting|CastToBaseCharacter_BP _returnvalue)
        (:then
          (if (Default|IsAlive _asbase_character_bp)
            (bind _outmodifiedamount (CallFunction|CalculateDifficultyMultiplier (Variables|UltimateCharacter|GetDamage) (Variables|Internal|GetDifficultyMultiplier) (Variables|Internal|GetGameDifficulty)))
            (LocalVariables|SetTempDamage _outmodifiedamount)
            (Debug|ShowDebugMessage "BaseBombard_BP" "CalculateDamage" (Utilities|String|Append (Utilities|String|ToString(Float) (LocalVariables|GetTempDamage)) " Damage to apply") "NewEnumerator0")
            (Attack|ApplyDamage (LocalVariables|GetTempDamage) InTarget)
            (else
              (Debug|ShowDebugMessage "BaseBombard_BP" "ApplyDamage" "Instigator is not alive" "NewEnumerator1"))))
        (:CastFailed
          (Debug|ShowDebugMessage "BaseBombard_BP" "ApplyDamage" "Cast failed to BaseCharacter_BP" "NewEnumerator2"))))
    (:Is%20Not%20Valid
      (Debug|ShowDebugMessage "BaseBombard_BP" "ApplyDamage" "Instigator is not valid" "NewEnumerator2"))))

(fn ShowDebugMessage
  (params (InCallerName :type String) (InFunction :type String) (InMessage :type String) (InMessageType :type MessageType%20Enum :default "NewEnumerator0"))
  (if (or (Variables|Debug|GetbShowDebug) (Utilities|Enum|Equal(Enum) InMessageType "NewEnumerator3"))
    (CallFunction|ShowDebugMessage InCallerName InFunction InMessage InMessageType)))

(fn FindAttackLocation
  (if (Variables|UltimateCharacter|GetbOwnerBase)
    ;[1 1 1] Use current attack owner location
    (return (Transformation|GetActorLocation (Game|GetInstigator)))
    (else
      ;[1 1 1] Find a random location near target to spawn attack
      (bind _asaicharacter_bp (Utilities|Casting|CastToAICharacter_BP (Game|GetInstigator))
        (:then
          (Utilities|IsValid (AI|GetBlackboard (Pawn|GetController _asaicharacter_bp))
            (:Is%20Valid
              (Utilities|IsValid (AI|Components|Blackboard|GetValueasObject (AI|GetBlackboard (Pawn|GetController _asaicharacter_bp)) (Utilities|Name|MakeLiteralName "Target"))
                (:Is%20Valid
                  (bind _asbase_character_bp (Utilities|Casting|CastToBaseCharacter_BP (AI|Components|Blackboard|GetValueasObject (AI|GetBlackboard (Pawn|GetController _asaicharacter_bp)) (Utilities|Name|MakeLiteralName "Target")))
                    (:then
                      (bind _randomlocation (Class|NavigationSystemV1|GetRandomLocationinNavigableRadius (Transformation|GetActorLocation _asbase_character_bp) (Variables|UltimateCharacter|GetNearTargetRadius) 0 0))
                      (LocalVariables|SetTempTargetLocation _randomlocation)
                      (Utilities|IsValid (Variables|UltimateCharacter|GetTargetLocationDecal)
                        (:Is%20Valid
                          (Rendering|Decal|SpawnDecalatLocation (Variables|UltimateCharacter|GetTargetLocationDecal) (Variables|UltimateCharacter|GetDecalSize) (- (LocalVariables|GetTempTargetLocation) (Math|Vector|MakeVector 0.0 0.0 (- (.z (Variables|UltimateCharacter|GetDecalSize)) 5.0))) "-90.000000,0.000000,0.000000" (Variables|UltimateCharacter|GetDecalLifeSpan)))
                        (:Is%20Not%20Valid
                          (Debug|ShowDebugMessage "BaseBombard_BP" "FindAttackLocation" "Decal material is not set to spawn decal at target" "NewEnumerator1")))
                      (return (LocalVariables|GetTempTargetLocation)))
                    (:CastFailed
                      (Debug|ShowDebugMessage "BaseBombard_BP" "FindAttackLocation" "Target is not child of BaseCharacter" "NewEnumerator2"))))
                (:Is%20Not%20Valid
                  (Debug|ShowDebugMessage "BaseBombard_BP" "FindAttackLocation" "Target is not valid" "NewEnumerator2"))))
            (:Is%20Not%20Valid
              (Debug|ShowDebugMessage "BaseBombard_BP" "FindAttackLocation" "Blackboard is not valid" "NewEnumerator2"))))
        (:CastFailed
          (bind _asplayer_character_bp (Utilities|Casting|CastToPlayerCharacter_BP (Game|GetInstigator))
            (:then
              (bind _randomlocation_2 (Class|NavigationSystemV1|GetRandomLocationinNavigableRadius (Default|GetCursorLocation _asplayer_character_bp) 1e+02 0 0))
              (return _randomlocation_2))
            (:CastFailed
              (Debug|ShowDebugMessage "BaseBombard_BP" "FindAttackLocation" "Cast to AI/Player character failed" "NewEnumerator2"))))))))

(fn ApplyDamage
  (params (InDamage :type Float%20%28double-precision%29) (InTarget :type Actor%20Object%20Reference))
  (bind _returnvalue (Game|GetInstigator))
  (Attack|ApplyForce InTarget)
  (Debug|ShowDebugMessage "BaseBombard_BP" "Apply Damage " (Utilities|String|Append "Apply " (Utilities|String|ToString(Float) InDamage) " damage using " (Utilities|String|SelectString "ApplyDamage function & Animate collision is enable" "ApplyRadialDamage & Animate collision is disable" (Variables|UltimateCharacter|GetbAnimateCollision))) "NewEnumerator0")
  (if (Variables|UltimateCharacter|GetbAnimateCollision)
    ;[1 1 1] Check if character can block the attack
    (bind _asbase_character_bp (Utilities|Casting|CastToBaseCharacter_BP InTarget))
    (bind (_boutblocked _outdamagepercent) (Default|DoBlockAttack _asbase_character_bp "NewEnumerator6"))
    (if _boutblocked
      (LocalVariables|SetTempDamagePercent _outdamagepercent))
    ;[1 1 1] Apply damage directly to actor
    (Game|Damage|ApplyDamage InTarget (/ (* (LocalVariables|GetTempDamagePercent) InDamage) 1e+02) (Pawn|GetController (Game|GetInstigator)) self (Variables|UltimateCharacter|GetDamageType))
    (else
      (bind _outactors (Attack|BlockCheck (Variables|UltimateCharacter|GetMaxDamageRadius)))
      (LocalVariables|SetTempIgnoreActors _outactors)
      (Utilities|Array|AddUnique (LocalVariables|GetTempIgnoreActors) _returnvalue)
      (Game|Damage|ApplyRadialDamage InDamage (select (Variables|UltimateCharacter|GetbOwnerBase) (Variables|Internal|GetTargetLocation) (Transformation|GetActorLocation)) (Variables|UltimateCharacter|GetMaxDamageRadius) (Variables|UltimateCharacter|GetDamageType) (LocalVariables|GetTempIgnoreActors) self (Pawn|GetController _returnvalue) (Variables|UltimateCharacter|GetbDoFullDamage) "ECC_Visibility")))
  (Utilities|IsValid (Variables|UltimateCharacter|GetExplodeEffect)
    (:Is%20Valid
      (Effects|SpawnEmitteratLocation (Variables|UltimateCharacter|GetExplodeEffect) (Transformation|GetActorLocation)))))

(fn DoAutoAttack
  (Debug|ShowDebugMessage "BaseBombard_BP" "DoAutoAttack" "" "NewEnumerator0")
  (Attack|CalculateDamage)
  (return))

(fn ApplyForce
  (params (InTarget :type Actor%20Object%20Reference))
  (Debug|ShowDebugMessage "BaseBombard_BP" "ApplyForce" (Utilities|String|SelectString (Utilities|String|Append "Apply force to " (Utilities|GetDisplayName InTarget)) "Apply force is not enable" (Variables|UltimateCharacter|GetbApplyForce)) "NewEnumerator0")
  (if (Variables|UltimateCharacter|GetbApplyForce)
    (bind _ascharacter (Utilities|Casting|CastToCharacter InTarget))
    (Physics|AddImpulse (Variables|/Script/Engine.Character|GetCharacterMovement _ascharacter) (* (Math|Vector|GetForwardVector (Math|Rotator|MakeRotator 0.0 0.0 (.yaw (Math|Rotator|FindLookatRotation (Transformation|GetActorLocation (Game|GetInstigator)) (Transformation|GetActorLocation _ascharacter))))) (Variables|UltimateCharacter|GetForce)) true)))

(fn BlockCheck
  (params (InRadius :type Float%20%28double-precision%29))
  ;[1 1 1] Get all characters
  (bind _outactors (Actor|GetAllActorsOfClass "/Game/UltimateCharacter/Blueprints/Characters/BaseCharacter_BP.BaseCharacter_BP_C"))
  (LocalVariables|SetTempAllCharacters _outactors)
  (Utilities|Array|RemoveItem (LocalVariables|GetTempAllCharacters) (.AsBase%20Character%20BP (Utilities|Casting|CastToBaseCharacter_BP (Game|GetInstigator))))
  ;[1 1 1] Check distance to target against suicide damage radius
  (for _array_element (LocalVariables|GetTempAllCharacters)
    (LocalVariables|SetTempTarget _array_element)
    (if (< (Math|Vector|VectorLength (- (Transformation|GetActorLocation self) (Transformation|GetActorLocation (LocalVariables|GetTempTarget)))) (* InRadius 2.0))
      ;[1 1 1] Check if something blocks the suicide explosion to the charachter
      (bind (_outhit _returnvalue) (Collision|LineTraceByChannel (Transformation|GetActorLocation) (Transformation|GetActorLocation (LocalVariables|GetTempTarget)) "TraceTypeQuery1" false (Utilities|Array|MakeArray self) "None"))
      (if _returnvalue
        (if (== (.HitActor (Collision|BreakHitResult _outhit)) (LocalVariables|GetTempTarget))
          ;[1 1 1] Run block function on target & if can block bombard attack add to ignore list
          (bind _boutblocked (Default|DoBlockAttack (LocalVariables|GetTempTarget) "NewEnumerator6" :!label _label))
          (if _boutblocked
            (Utilities|Array|AddUnique (LocalVariables|GetTempCharacters) (LocalVariables|GetTempTarget)))
          (else
            (Debug|ShowDebugMessage "BaseBombard_BP" "BlockCheck" (Utilities|String|Append (Utilities|GetDisplayName (.HitActor (Collision|BreakHitResult _outhit))) " blocks sight from " (Utilities|GetDisplayName self) " suicide damage to " (Utilities|GetDisplayName (LocalVariables|GetTempTarget))) "NewEnumerator3")))
        (else
          (goto _label)))))
  (return (LocalVariables|GetTempCharacters)))