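; Kwang's sword bombard Blueprint, a child of a bombard parent that adds an animated sword effect.
; Before the bombard is enabled, it runs the parent logic, then plays a timeline that lowers the Sword along relative Z while scaling it up from zero.
; On completion, a short delay reverses the timeline to raise and shrink the sword, with a DoOnce preventing repeated reversal.
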(event EventBeginPlay
  (|CallParentFunction) ; This node is disabled and will not be called.\nDrag off pins to build functionality.
)

(event Collision|EventActorBeginOverlap
  (params (OtherActor :type Actor%20Object%20Reference)))

(event EventTick
  (params (DeltaSeconds :type Float%20%28single-precision%29)))

(event EventBeforeEnableBombard
  ;[1 1 1] Animate sword effect
  (|CallParentFunction)
  (bind (_direction _alphalocation _alphascale) (Timeline|SwordAnimation PlayFromStart)
    (:Update
      (Transformation|SetRelativeLocation (Variables|Default|GetSword) (Math|Vector|Lerp(Vector) "0, 0,310.000000" "0.000000, 0,150.000000" _alphalocation) false false)
      (Transformation|SetWorldScale3D (Variables|Default|GetSword) (Math|Vector|Lerp(Vector) "0, 0, 0" "1.000000,1.000000,1.000000" _alphascale)))
    (:Finished
      (Utilities|FlowControl|DoOnce false
        (:Completed
          (Utilities|FlowControl|Delay 0.3)
          (Timeline|SwordAnimation ReverseFromEnd))))))

(fn ConstructionScript
  (|CallParentFunction))