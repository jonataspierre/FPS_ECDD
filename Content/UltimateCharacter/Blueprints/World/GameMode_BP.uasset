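; Game mode Blueprint that sets combat damage rules, exposes game difficulty and chooses the player pawn class.
; ModifyDamage zeroes damage between same-team characters by comparing PlayerState_BP team numbers through CanDealDamage, and passes it through unchanged when those references are missing.
; GetDefaultPawnClassForController prefers the character class stored in GameInstance_BP, falling back to the parent's choice.
; Killed only resolves killer and victim player states, with no further logic.
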(event EventBeginPlay)

(event EventTick
  (params (DeltaSeconds :type Float%20%28single-precision%29)))

(fn ConstructionScript)

(fn GetDifficulty
  (return (Variables|Default|GetGameDifficulty)))

(fn CanDealDamage
  (params (InDamageInstigator :type Player%20State%20BP%20Object%20Reference) (InDamagedCharacter :type Player%20State%20BP%20Object%20Reference))
  ;[1 1 1] Check team number to see if characters are enemy or not
  (Utilities|IsValid InDamageInstigator
    (:Is%20Valid
      (Utilities|IsValid InDamagedCharacter
        (:Is%20Valid
          (return (not (== (Default|GetTeamNumber InDamageInstigator) (Default|GetTeamNumber InDamagedCharacter)))))
        (:Is%20Not%20Valid
          (return true))))
    (:Is%20Not%20Valid
      (return true))))

(fn ModifyDamage
  (params (InDamage :type Float%20%28double-precision%29) (InDamagedActor :type Actor%20Object%20Reference) (InEventInstigator :type Controller%20Object%20Reference) (InDamageCause :type Actor%20Object%20Reference))
  (bind _playerstate (Variables|/Script/Engine.Controller|GetPlayerState InEventInstigator))
  (bind (_asplayer_state_bp _bsuccess) (Utilities|Casting|CastToPlayerState_BP _playerstate))
  (LocalVariables|SetTempActualDamage InDamage)
  (bind _asbase_character_bp (Utilities|Casting|CastToBaseCharacter_BP InDamagedActor)
    (:then
      (bind _output_get (LocalVariables|SetTempDamagedPawn _asbase_character_bp))
      (Utilities|IsValid _output_get
        (:Is%20Valid
          (Utilities|IsValid InEventInstigator
            (:Is%20Valid
              (LocalVariables|SetTempInPS _asplayer_state_bp)
              (LocalVariables|SetTempPS (.AsPlayer%20State%20BP (Utilities|Casting|CastToPlayerState_BP (Variables|/Script/Engine.Pawn|GetPlayerState (LocalVariables|GetTempDamagedPawn)))))
              (if (and _bsuccess (.bSuccess (Utilities|Casting|CastToPlayerState_BP (Variables|/Script/Engine.Pawn|GetPlayerState (LocalVariables|GetTempDamagedPawn)))))
                (bind _bdamage (CallFunction|CanDealDamage (LocalVariables|GetTempInPS) (LocalVariables|GetTempPS)))
                (if _bdamage
                  (return (LocalVariables|GetTempActualDamage))
                  (else
                    (return 0.0)))
                (else
                  (return (LocalVariables|GetTempActualDamage)))))
            (:Is%20Not%20Valid
              (return (LocalVariables|GetTempActualDamage)))))
        (:Is%20Not%20Valid
          (return (LocalVariables|GetTempActualDamage)))))
    (:CastFailed
      (return (LocalVariables|GetTempActualDamage)))))

(fn Killed
  (params (InKiller :type Controller%20Object%20Reference) (InKilledPlayer :type Controller%20Object%20Reference) (InKilledPawn :type Pawn%20Object%20Reference) (InDmgType :type Damage%20Type%20Object%20Reference))
  (bind _playerstate (Variables|/Script/Engine.Controller|GetPlayerState InKiller))
  (bind _playerstate_2 (Variables|/Script/Engine.Controller|GetPlayerState InKilledPlayer))
  (bind (_asplayer_state_bp _bsuccess) (Utilities|Casting|CastToPlayerState_BP _playerstate))
  (bind (_asplayer_state_bp_2 _bsuccess_2) (Utilities|Casting|CastToPlayerState_BP _playerstate_2))
  (Utilities|IsValid InKiller
    (:Is%20Valid
      (LocalVariables|SetKillerPlayerState _asplayer_state_bp))
    (:Is%20Not%20Valid
      _))
  (Utilities|IsValid InKilledPlayer
    (:Is%20Valid
      (LocalVariables|SetKilledPlayerState _asplayer_state_bp_2)
      (if (and _bsuccess _bsuccess_2)
        _))))

(fn GetDefaultPawnClassforController
  (params (InController :type Controller%20Object%20Reference))
  (bind _returnvalue (|CallParentFunction InController))
  (LocalVariables|SetTempPawnClass _returnvalue)
  (bind _asgame_instance_bp (Utilities|Casting|CastToGameInstance_BP (Game|GetGameInstance))
    (:then
      (return (select (Utilities|IsValidClass (Variables|/Game/UltimateCharacter/Blueprints/World/GameInstance_BP.GameInstance_BP_C|GetPlayerCharacterClass _asgame_instance_bp)) (Variables|/Game/UltimateCharacter/Blueprints/World/GameInstance_BP.GameInstance_BP_C|GetPlayerCharacterClass _asgame_instance_bp) (LocalVariables|GetTempPawnClass))))
    (:CastFailed
      (return (LocalVariables|GetTempPawnClass)))))