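; AI controller for AICharacter_BP enemies that starts their behavior tree and exposes blackboard getters and setters for combat state.
; Perception sets or clears an enemy target, recording its last location, starting a recognition-reset timer and flagging a pickup search on low health.
; Heard noises set a randomized investigate point, re-triggering through a short delay if already active.
; It also manages attack type and counter, player block windows, team number and checkpoint reset.
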(event OnTargetPerceptionUpdated(AIPerception)
  (params (Actor :type Actor%20Object%20Reference) (Stimulus :type AI%20Stimulus%20Structure))
  ;[1 1 1] Perception update
  (AI|OnCharacterPerceptionUpdate Actor Stimulus))

(event OnHearNoise(PawnSensing)
  (params (Instigator :type Pawn%20Object%20Reference) (Location :type Vector%20%28by%20ref%29 :default "0, 0, 0") (Volume :type Float%20%28single-precision%29))
  ;[1 1 1] Character hear noise
  (AI|OnCharacterHear Instigator Location Volume))

(event EventBeginPlay
  (bind _behaviortreeclass (Variables|UltimateCharacter-AIConfig|GetBehaviorTreeClass))
  (bind _blackboardclass (Variables|UltimateCharacter-AIConfig|GetBlackboardClass))
  ;[1 1 1] Beginplay event to do some initialization
  (AI|UpdateTeamNumber (Variables|UltimateCharacter-AIConfig|GetTeamNumber))
  ;;[1 1 1] Run behavior tree and blackboard
  (Utilities|IsValid _blackboardclass
    (:Is%20Valid
      (AI|SetBlackboard _blackboardclass)
      (Utilities|IsValid _behaviortreeclass
        (:Is%20Valid
          (AI|StartBT _behaviortreeclass))
        (:Is%20Not%20Valid
          (Debug|ShowDebugMessage "BaseAIController_BP" "BeginPlay" "BehaviorTree is not valid" "NewEnumerator2"))))
    (:Is%20Not%20Valid
      (Debug|ShowDebugMessage "BaseAIController_BP" "BeginPlay" "Blackboard is not valid" "NewEnumerator2"))))

(event EventPossess
  (params (PossessedPawn :type Pawn%20Object%20Reference))
  ;[1 1 1] Possess & Unpossess character
  (bind _asaicharacter_bp (Utilities|Casting|CastToAICharacter_BP PossessedPawn)
    (:then
      (Variables|Internal|SetPawn_AI _asaicharacter_bp))
    (:CastFailed
      (Debug|ShowDebugMessage "BaseAIController_BP" "BeginPlay" "PawnAI is not valid" "NewEnumerator3"))))

(event EventUnPossess
  (params (UnpossessedPawn :type Pawn%20Object%20Reference))
  ;[1 1 1] Possess & Unpossess character
  (Variables|Internal|SetPawn_AI 0)
  (AI|Logic|StopLogic (Variables|Default|GetBrainComponent) ""))

(fn ConstructionScript)

(fn SetBlackboard
  (params (InBlackboardAsset :type Blackboard%20Data%20Object%20Reference))
  (bind _blackboardcomponent (Class|AIController|UseBlackboard InBlackboardAsset))
  (AI|Components|Blackboard|SetValueasVector _blackboardcomponent (Utilities|Name|MakeLiteralName "LastSeenLocation") "0, 0, 0"))

(fn StartBT
  (params (InBTAsset :type Behavior%20Tree%20Object%20Reference))
  (AI|RunBehaviorTree InBTAsset))

(fn GetDistanceforAttack
  (params (InAttackType :type AttackTypes_AI%20Enum :default "NewEnumerator5") (InDistanceToTarget :type Float%20%28double-precision%29))
  ;[1 1 1] Try to read distance from pawn if do not store any distance range for current attack
  (if (Utilities|Enum|Equal(Enum) InAttackType (Variables|Internal|GetLastAttackType))
    _
    (else
      (Variables|Internal|SetLastAttackType InAttackType)
      (Variables|Internal|SetRange (Default|GetAttackRange (Variables|Internal|GetPawn_AI) InAttackType))))
  ;[1 1 1] Check to see if distance to target is in attack range or not
  (return (and (>= InDistanceToTarget (.Value (Utilities|Struct|BreakFloatRangeBound (.LowerBound (Utilities|Struct|BreakFloatRange (Variables|Internal|GetRange)))))) (<= InDistanceToTarget (.Value (Utilities|Struct|BreakFloatRangeBound (.UpperBound (Utilities|Struct|BreakFloatRange (Variables|Internal|GetRange))))))) (Variables|Internal|GetRange)))

(fn SetAttackTypes
  (params (InAttacks :type Array%20of%20AttackTypes_AI%20Enums :default "NewEnumerator5"))
  ;[1 1 1] This function will call from AICharacter_BP at begin play to create an unique attack types array
  (Debug|ShowDebugMessage "BaseAIController_BP" "SetAttackTypes" (Utilities|String|ToString(Name) (Variables|/Game/UltimateCharacter/Blueprints/Characters/BaseCharacter_BP.BaseCharacter_BP_C|GetCharacterTag (Variables|Internal|GetPawn_AI))) "NewEnumerator0")
  (for _array_element InAttacks
    (Utilities|Array|AddUnique (Variables|Internal|GetAttackTypes) _array_element)))

(fn GetTarget
  (bind _asbase_character_bp (Utilities|Casting|CastToBaseCharacter_BP (AI|Components|Blackboard|GetValueasObject (AI|GetBlackboard 0) (Utilities|Name|MakeLiteralName "Target")))
    (:then
      (return _asbase_character_bp))
    (:CastFailed
      (return 0))))

(fn ShowDebugMessage
  (params (InCallerName :type String) (InFunction :type String) (InMessage :type String) (InMessageType :type MessageType%20Enum :default "NewEnumerator0"))
  (if (or (Variables|UltimateCharacter-Debug|GetbShowDebugMessage) (Utilities|Enum|Equal(Enum) InMessageType "NewEnumerator3"))
    (CallFunction|ShowDebugMessage InCallerName InFunction InMessage InMessageType)))

(fn UpdateTeamNumber
  (params (InTeam :type Integer))
  (Variables|UltimateCharacter-AIConfig|SetTeamNumber InTeam)
  (bind _asplayer_state_bp (Utilities|Casting|CastToPlayerState_BP (Variables|GetPlayerState))
    (:then
      (Default|SetTeamNumber _asplayer_state_bp (Variables|UltimateCharacter-AIConfig|GetTeamNumber)))
    (:CastFailed
      (Debug|ShowDebugMessage "BaseAIController_BP" "UpdateTeamNumber" "Cast to PlayerState_BP failed" "NewEnumerator2"))))

(fn OnCharacterPerceptionUpdate
  (params (InActor :type Actor%20Object%20Reference) (InAIStimulus :type AI%20Stimulus%20Structure))
  (bind _outtarget (GetInfo|GetTarget))
  (bind _pawn_ai (Variables|Internal|GetPawn_AI))
  (Utilities|IsValid (Variables|Internal|GetPawn_AI)
    (:Is%20Valid
      (Utilities|IsValid InActor
        (:Is%20Valid
          (bind _asbase_character_bp (Utilities|Casting|CastToBaseCharacter_BP InActor))
          (if (Default|IsEnemyfor _asbase_character_bp self)
            (if (Utilities|Struct|BreakAIStimulus InAIStimulus)
              (Utilities|IsValid _outtarget
                (:Is%20Valid
                  (if (not (== _outtarget InActor))
                    (Debug|ShowDebugMessage "BaseAIController_BP" "OnCharacterPerceptionUpdate" "TODO : We already have a target what to do with a new target?" "NewEnumerator2")))
                (:Is%20Not%20Valid
                  (SetInfo|SetTarget InActor)
                  (Utilities|Time|ClearandInvalidateTimerbyHandle (Variables|Internal|GetResetRecognizeTimer))
                  (Utilities|Time|ClearandInvalidateTimerbyHandle (Variables|Internal|GetHeardResetTimer))
                  (SetInfo|ResetHeardNoise)
                  (Debug|ShowDebugMessage "BaseAIController_BP" "OnCharacterPerceptionUpdate" (Utilities|String|Append "New target is set in BB for " (Utilities|String|ToString(Name) (Variables|/Game/UltimateCharacter/Blueprints/Characters/BaseCharacter_BP.BaseCharacter_BP_C|GetCharacterTag (Variables|Internal|GetPawn_AI)))) "NewEnumerator0")))
              (else
                ;[1 1 1] Reset target & set last seen location
                (SetInfo|SetTarget)
                (AI|Components|Blackboard|SetValueasVector (AI|GetBlackboard 0) (Utilities|Name|MakeLiteralName "LastTargetLocation") (Utilities|Struct|BreakAIStimulus InAIStimulus))
                (Debug|ShowDebugMessage "BaseAIController_BP" "OnCharacterPerceptionUpdate" (Utilities|String|Append "Target ia removed from BB for " (Utilities|String|ToString(Name) (Variables|/Game/UltimateCharacter/Blueprints/Characters/BaseCharacter_BP.BaseCharacter_BP_C|GetCharacterTag (Variables|Internal|GetPawn_AI)))) "NewEnumerator0")
                (AI|CheckforHealth 4e+01)
                ;[1 1 1] Set timer for reset remaining recognize time for next time seeing the enemy
                (if (and (!= (Class|BlackboardComponent|GetValueasFloat (AI|GetBlackboard 0) (Utilities|Name|MakeLiteralName "RemainRecognizeTime")) 0.0) (Default|IsAlive _pawn_ai))
                  (bind _returnvalue (Utilities|Time|SetTimerbyFunctionName self "ResetRemainingRecognizeTime" (Utilities|Struct|BreakAI_Recognize_Struct (Utilities|Struct|BreakAI_Configs_Struct (Variables|/Game/UltimateCharacter/Blueprints/Characters/AICharacter_BP.AICharacter_BP_C|GetAIConfig _pawn_ai)))))
                  (Variables|Internal|SetResetRecognizeTimer _returnvalue))))))
        (:Is%20Not%20Valid
          (Debug|ShowDebugMessage "BaseAIController_BP" "OnCharacterPerceptionUpdate" "Pawn is not valid" "NewEnumerator2" :!label _label))))
    (:Is%20Not%20Valid
      (goto _label))))

(fn ResetRemainingRecognizeTime
  (Utilities|IsValid (Variables|Internal|GetPawn_AI)
    (:Is%20Valid
      (Debug|ShowDebugMessage "BaseAIController_BP" "ResetRemainingRecognizeTime" (Utilities|String|ToString(Name) (Variables|/Game/UltimateCharacter/Blueprints/Characters/BaseCharacter_BP.BaseCharacter_BP_C|GetCharacterTag (Variables|Internal|GetPawn_AI))) "NewEnumerator0")
      ;[1 1 1] Reset remaining time so next time recognize starts from begining and reset the widget
      (AI|Components|Blackboard|SetValueasFloat (AI|GetBlackboard 0) (Utilities|Name|MakeLiteralName "RemainRecognizeTime") 0.0)
      (Default|UpdateRecognitionBar (Variables|Internal|GetPawn_AI) 1.1))))

(fn InitializeDefaultAttack
  (params (InAttackType :type AttackTypes_AI%20Enum :default "NewEnumerator5") (InTag :type Name) (InCounter :type Integer))
  (bind _returnvalue (AI|GetBlackboard 0))
  (Debug|ShowDebugMessage "BaseAIController_BP" "InitializeDefaultAttackType" (Utilities|String|Append (Utilities|String|EnumtoString InAttackType) " for " (Utilities|String|ToString(Name) (Variables|/Game/UltimateCharacter/Blueprints/Characters/BaseCharacter_BP.BaseCharacter_BP_C|GetCharacterTag (Variables|Internal|GetPawn_AI)))) "NewEnumerator0")
  (Utilities|IsValid _returnvalue
    (:Is%20Valid
      (LocalVariables|SetTempBB _returnvalue)
      (if (> (Utilities|Array|Length (Variables|Internal|GetAttackTypes)) 0)
        ;[1 1 1] Set default attack type
        (if (== (Utilities|Array|Length (Variables|Internal|GetAttackTypes)) 1)
          (AI|Components|Blackboard|SetValueasEnum (LocalVariables|GetTempBB) (Utilities|Name|MakeLiteralName "CurrentAttackType") (Utilities|Array|Get(acopy) (Variables|Internal|GetAttackTypes)))
          ;[1 1 1] Set attack counter & attack tag
          (Class|BlackboardComponent|SetValueasInt (LocalVariables|GetTempBB) (Utilities|Name|MakeLiteralName "AttackCounter") InCounter :!label _label)
          (Class|BlackboardComponent|SetValueasName (LocalVariables|GetTempBB) (Utilities|Name|MakeLiteralName "AttackTag") InTag)
          (elif (!= (Utilities|Array|FindItem (Variables|Internal|GetAttackTypes) InAttackType) -1)
            (AI|Components|Blackboard|SetValueasEnum (LocalVariables|GetTempBB) (Utilities|Name|MakeLiteralName "CurrentAttackType") InAttackType)
            (goto _label)
            (else
              (Debug|ShowDebugMessage "BaseAIController_BP" "InitializeDefaultAttackType" "Attack type not found" "NewEnumerator3"))))
        (else
          (Debug|ShowDebugMessage "BaseAIController_BP" "InitializeDefaultAttackType" "Attack types not found" "NewEnumerator3"))))
    (:Is%20Not%20Valid
      (Debug|ShowDebugMessage "BaseAIController_BP" "InitializeDefaultAttackType" "Blackboard is not valid" "NewEnumerator3"))))

(fn UpdateAttackCounter
  (bind _returnvalue (AI|GetBlackboard 0))
  (Utilities|IsValid (Variables|Internal|GetPawn_AI)
    (:Is%20Valid
      (Debug|ShowDebugMessage "BaseAIController_BP" "UpdateAttackCounter" (Utilities|String|ToString(Name) (Variables|/Game/UltimateCharacter/Blueprints/Characters/BaseCharacter_BP.BaseCharacter_BP_C|GetCharacterTag (Variables|Internal|GetPawn_AI))) "NewEnumerator0")
      (if (Variables|/Game/UltimateCharacter/Blueprints/Characters/AICharacter_BP.AICharacter_BP_C|GetDynamicAttacks (Variables|Internal|GetPawn_AI))
        ;[1 1 1] Reduce attack count after each attack
        (Utilities|IsValid _returnvalue
          (:Is%20Valid
            (LocalVariables|SetTempAttackCount (Class|BlackboardComponent|GetValueasInt _returnvalue (Utilities|Name|MakeLiteralName "AttackCounter")))
            (Class|BlackboardComponent|SetValueasInt (AI|GetBlackboard 0) (Utilities|Name|MakeLiteralName "AttackCounter") (- (LocalVariables|GetTempAttackCount) 1))
            (return (> (- (LocalVariables|GetTempAttackCount) 1) 0)))
          (:Is%20Not%20Valid
            (return false)))
        (else
          (Debug|ShowDebugMessage "BaseAIController_BP" "UpdateAttackCounter" (Utilities|String|Append (Utilities|String|ToString(Name) (Variables|/Game/UltimateCharacter/Blueprints/Characters/BaseCharacter_BP.BaseCharacter_BP_C|GetCharacterTag (Variables|Internal|GetPawn_AI))) ", dynamic attack is not active and attack will not change until out of ammo") "NewEnumerator1")
          (return true))))))

(fn OnCharacterHear
  (params (InPawnInstigator :type Pawn%20Object%20Reference) (InLocation :type Vector) (InVolume :type Float%20%28double-precision%29))
  (Utilities|IsValid (Variables|Internal|GetPawn_AI)
    (:Is%20Valid
      (Debug|ShowDebugMessage "BaseAIController_BP" "OnCharacterHear" (Utilities|String|ToString(Name) (Variables|/Game/UltimateCharacter/Blueprints/Characters/BaseCharacter_BP.BaseCharacter_BP_C|GetCharacterTag (Variables|Internal|GetPawn_AI))) "NewEnumerator0")
      ;[1 1 1] Check blackboard, check character and any exsiting target
      (Utilities|IsValid (GetInfo|GetTarget) ; Don't check heard noise instigator if target is set
        (:Is%20Not%20Valid
          (bind _asbase_character_bp (Utilities|Casting|CastToBaseCharacter_BP InPawnInstigator)
            (:then
              (if (GetInfo|GetHeardSomthing)
                ;[1 1 1] Try to trigger manually the hear tree
                (SetInfo|SetHeardNoise false)
                (Utilities|Time|SetTimerbyFunctionName self "ForceHearSomething" 0.5)
                (Variables|Internal|SetHPawn InPawnInstigator)
                (Variables|Internal|SetHLocation InLocation)
                (Variables|Internal|SetHVolume InVolume)
                (else
                  (Variables|Internal|SetHPawn 0)
                  (Variables|Internal|SetHLocation "0, 0, 0")
                  (Variables|Internal|SetHVolume 0.0)
                  (SetInfo|SetHeardNoise true)
                  (LocalVariables|SetbTempEnemy (Default|IsEnemyfor _asbase_character_bp self))
                  (AI|Components|Blackboard|SetValueasBool (AI|GetBlackboard 0) (Utilities|Name|MakeLiteralName "bHeardEnemy") (LocalVariables|GetbTempEnemy))
                  ;[1 1 1] Set move to location for noise heard location
                  (bind _randomlocation (Class|NavigationSystemV1|GetRandomLocationinNavigableRadius InLocation (Math|Float|SelectFloat (Math|Float|MapRangeClamped InVolume 1.0 0.0 2e+02 5e+02) 5e+02 (LocalVariables|GetbTempEnemy)) 0 0))
                  (AI|Components|Blackboard|SetValueasVector (AI|GetBlackboard 0) (Utilities|Name|MakeLiteralName "MoveToLocation") _randomlocation)
                  ;[1 1 1] Handle reseting heard noise
                  (Utilities|Time|ClearandInvalidateTimerbyHandle (Variables|Internal|GetHeardResetTimer))
                  (bind _returnvalue (Utilities|Time|SetTimerbyFunctionName self "ResetHeardNoise" (Variables|UltimateCharacter-AIConfig|GetSoundRemembering)))
                  (Variables|Internal|SetHeardResetTimer _returnvalue))))
            (:CastFailed
              (Debug|ShowDebugMessage "BaseAIController_BP" "OnCharacterHear" "Instigator is not character" "NewEnumerator2"))))))))

(fn ResetHeardNoise
  (Utilities|IsValid (Variables|Internal|GetPawn_AI)
    (:Is%20Valid
      (Debug|ShowDebugMessage "BaseAIController_BP" "ResetHeardNoise" (Utilities|String|ToString(Name) (Variables|/Game/UltimateCharacter/Blueprints/Characters/BaseCharacter_BP.BaseCharacter_BP_C|GetCharacterTag (Variables|Internal|GetPawn_AI))) "NewEnumerator0")
      (AI|Components|Blackboard|SetValueasBool (AI|GetBlackboard 0) (Utilities|Name|MakeLiteralName "bHeardSomething") false))))

(fn SetChangeAttack
  (params (InChange :type Boolean))
  (Utilities|IsValid (Variables|Internal|GetPawn_AI)
    (:Is%20Valid
      (Debug|ShowDebugMessage "BaseAIController_BP" "ChangeAttack" (Utilities|String|ToString(Name) (Variables|/Game/UltimateCharacter/Blueprints/Characters/BaseCharacter_BP.BaseCharacter_BP_C|GetCharacterTag (Variables|Internal|GetPawn_AI))) "NewEnumerator0")
      ;[1 1 1] Update change attack state & Attack counter in BB
      (AI|Components|Blackboard|SetValueasBool (AI|GetBlackboard 0) (Utilities|Name|MakeLiteralName "bChangeAttack") InChange)
      (Class|BlackboardComponent|SetValueasInt (AI|GetBlackboard 0) (Utilities|Name|MakeLiteralName "AttackCounter")))))

(fn ActivatePlayerBlock
  (params (InConfig :type Player%20Block%20Config%20Struct%20Structure))
  (Debug|ShowDebugMessage "BaseAIController_BP" "ActivatePlayerBlock" (Utilities|String|ToString(Name) (Variables|/Game/UltimateCharacter/Blueprints/Characters/BaseCharacter_BP.BaseCharacter_BP_C|GetCharacterTag (Variables|Internal|GetPawn_AI))) "NewEnumerator0")
  ;[1 1 1] Set incoming attack block config on player to be able to block the attack
  (bind _asplayer_character_bp (Utilities|Casting|CastToPlayerCharacter_BP (GetInfo|GetTarget)))
  (if (not (Utilities|Time|IsTimerActivebyHandle (Variables|/Game/UltimateCharacter/Blueprints/Characters/PlayerCharacter_BP.PlayerCharacter_BP_C|GetBlockResetTimer _asplayer_character_bp)))
    (Default|SetBlockConfig _asplayer_character_bp InConfig (Variables|Internal|GetPawn_AI))))

(fn SetBlockingState
  (params (InBlock :type Boolean))
  (Utilities|IsValid (Variables|Internal|GetPawn_AI)
    (:Is%20Valid
      (Debug|ShowDebugMessage "BaseAIController_BP" "SetBlockingState" (Utilities|String|ToString(Name) (Variables|/Game/UltimateCharacter/Blueprints/Characters/BaseCharacter_BP.BaseCharacter_BP_C|GetCharacterTag (Variables|Internal|GetPawn_AI))) "NewEnumerator0")
      ;[1 1 1] Update blocking state in BB
      (AI|Components|Blackboard|SetValueasBool (AI|GetBlackboard 0) (Utilities|Name|MakeLiteralName "bBlockIncomingAttack") InBlock))))

(fn SetLastHit
  (params (InHit :type Boolean))
  (bind _pawn_ai (Variables|Internal|GetPawn_AI))
  (Utilities|IsValid _pawn_ai
    (:Is%20Valid
      (Debug|ShowDebugMessage "BaseAIController_BP" "SetLastHit" (Utilities|String|ToString(Name) (Variables|/Game/UltimateCharacter/Blueprints/Characters/BaseCharacter_BP.BaseCharacter_BP_C|GetCharacterTag _pawn_ai)) "NewEnumerator0"))
    (:Is%20Not%20Valid
      _))
  ;[1 1 1] Update blocking state in BB
  (AI|Components|Blackboard|SetValueasBool (AI|GetBlackboard 0) (Utilities|Name|MakeLiteralName "bHitInLastAttack") InHit))

(fn GetAttackType
  (return (Utilities|Enum|ByteToEnumAttackTypes_AI (Class|BlackboardComponent|GetValueasEnum (AI|GetBlackboard 0) (Utilities|Name|MakeLiteralName "CurrentAttackType")))))

(fn GetAttackTag
  (return (Class|BlackboardComponent|GetValueasName (AI|GetBlackboard 0) (Utilities|Name|MakeLiteralName "AttackTag"))))

(fn GetIsinAttack
  (return (ScalableFloat|GetValueasBool (AI|GetBlackboard 0) (Utilities|Name|MakeLiteralName "bIsAttacking"))))

(fn GetHitLastAttack
  (return (ScalableFloat|GetValueasBool (AI|GetBlackboard 0) (Utilities|Name|MakeLiteralName "bHitInLastAttack"))))

(fn SetRemainigRecognizeTime
  (params (InTime :type Float%20%28double-precision%29))
  (bind _pawn_ai (Variables|Internal|GetPawn_AI))
  (Utilities|IsValid _pawn_ai
    (:Is%20Valid
      (Debug|ShowDebugMessage "BaseAIController_BP" "SetRemainigRecognizeTime" (Utilities|String|ToString(Name) (Variables|/Game/UltimateCharacter/Blueprints/Characters/BaseCharacter_BP.BaseCharacter_BP_C|GetCharacterTag _pawn_ai)) "NewEnumerator0")
      ;[1 1 1] Update remaining time to recognize target BB
      (AI|Components|Blackboard|SetValueasFloat (AI|GetBlackboard 0) (Utilities|Name|MakeLiteralName "SetRemainigRecognizeTime") InTime))))

(fn SetForceRecognize
  (params (InRecognize :type Boolean))
  (Utilities|IsValid (Variables|Internal|GetPawn_AI)
    (:Is%20Valid
      (Debug|ShowDebugMessage "BaseAIController_BP" "SetForceRecognize" (Utilities|String|ToString(Name) (Variables|/Game/UltimateCharacter/Blueprints/Characters/BaseCharacter_BP.BaseCharacter_BP_C|GetCharacterTag (Variables|Internal|GetPawn_AI))) "NewEnumerator0")
      ;[1 1 1] Update force recognize in BB
      (AI|Components|Blackboard|SetValueasBool (AI|GetBlackboard 0) (Utilities|Name|MakeLiteralName "bDoRecognize") InRecognize))))

(fn GetLastTargetLocation
  (return (AI|Components|Blackboard|GetValueasVector (AI|GetBlackboard 0) (Utilities|Name|MakeLiteralName "LastTargetLocation"))))

(fn GetHeardSomthing
  (return (ScalableFloat|GetValueasBool (AI|GetBlackboard 0) (Utilities|Name|MakeLiteralName "bHeardSomething"))))

(fn SetHeardNoise
  (params (InHeard :type Boolean))
  (Utilities|IsValid (Variables|Internal|GetPawn_AI)
    (:Is%20Valid
      (Debug|ShowDebugMessage "BaseAIController_BP" "SetHeardNoise" (Utilities|String|ToString(Name) (Variables|/Game/UltimateCharacter/Blueprints/Characters/BaseCharacter_BP.BaseCharacter_BP_C|GetCharacterTag (Variables|Internal|GetPawn_AI))) "NewEnumerator0")
      (AI|Components|Blackboard|SetValueasBool (AI|GetBlackboard 0) (Utilities|Name|MakeLiteralName "bHeardSomething") InHeard))))

(fn ForceHearSomething
  (AI|OnCharacterHear (Variables|Internal|GetHPawn) (Variables|Internal|GetHLocation) (Variables|Internal|GetHVolume)))

(fn SetTarget
  (params (InObject :type Object%20Object%20Reference))
  (Utilities|IsValid (Variables|Internal|GetPawn_AI)
    (:Is%20Valid
      (Debug|ShowDebugMessage "BaseAIController_BP" "SetTarget" (Utilities|String|ToString(Name) (Variables|/Game/UltimateCharacter/Blueprints/Characters/BaseCharacter_BP.BaseCharacter_BP_C|GetCharacterTag (Variables|Internal|GetPawn_AI))) "NewEnumerator0")
      (AI|Components|Blackboard|SetValueasObject (AI|GetBlackboard 0) (Utilities|Name|MakeLiteralName "Target") InObject))))

(fn GetRemainingRecognizeTime
  (return (Class|BlackboardComponent|GetValueasFloat (AI|GetBlackboard 0) (Utilities|Name|MakeLiteralName "RemainRecognizeTime"))))

(fn ForceAttackChange
  (params (InAttackType :type AttackTypes_AI%20Enum :default "NewEnumerator5") (InAttackTag :type Name) (InAttackCount :type Integer))
  (Utilities|IsValid (Variables|Internal|GetPawn_AI)
    (:Is%20Valid
      (Debug|ShowDebugMessage "BaseAIController_BP" "ForceAttackChange" (Utilities|String|Append "New Attack : " (Utilities|String|EnumtoString InAttackType) ", New Attack Tag : " (Utilities|String|ToString(Name) InAttackTag) ", New Attack Count : " (Utilities|String|ToString(Integer) InAttackCount) ", for " (Utilities|String|ToString(Name) (Variables|/Game/UltimateCharacter/Blueprints/Characters/BaseCharacter_BP.BaseCharacter_BP_C|GetCharacterTag (Variables|Internal|GetPawn_AI)))) "NewEnumerator0")
      (Class|BlackboardComponent|SetValueasInt (AI|GetBlackboard 0) (Utilities|Name|MakeLiteralName "AttackCounter") (Math|Integer|Absolute(Integer) InAttackCount))
      (Class|BlackboardComponent|SetValueasName (AI|GetBlackboard 0) (Utilities|Name|MakeLiteralName "AttackTag") InAttackTag)
      (AI|Components|Blackboard|SetValueasEnum (AI|GetBlackboard 0) (Utilities|Name|MakeLiteralName "CurrentAttackType") InAttackType))))

(fn CheckforHealth
  (params (InThreshold :type Float%20%28double-precision%29))
  (bind _pawn_ai (Variables|Internal|GetPawn_AI))
  (Debug|ShowDebugMessage "BaseAIController_BP" "CheckForHealth" (Utilities|String|Append "Threshold for health percent is " (Utilities|String|ToString(Float) InThreshold)) "NewEnumerator0")
  ;[1 1 1] Calculate the check current health percent against threshold
  (LocalVariables|SetTempPercent (Math|Float|Clamp(Float) (Math|Float|Absolute(Float) InThreshold) 0.0 1e+02))
  (if (< (/ (* (Default|GetHealth _pawn_ai) 1e+02) (Variables|/Game/UltimateCharacter/Blueprints/Characters/BaseCharacter_BP.BaseCharacter_BP_C|GetMaxHealth _pawn_ai)) (LocalVariables|GetTempPercent))
    (AI|Components|Blackboard|SetValueasEnum (AI|GetBlackboard 0) (Utilities|Name|MakeLiteralName "PickupSearch") (Utilities|Enum|LiteralenumPickupList_Enum "NewEnumerator1"))))

(fn CheckpointReset
  (bind _pawn_ai (Variables|Internal|GetPawn_AI))
  (Utilities|IsValid (Variables|Internal|GetPawn_AI)
    (:Is%20Valid
      (Debug|ShowDebugMessage "BaseAIController_BP" "CheckpointReset" (Utilities|String|ToString(Name) (Variables|/Game/UltimateCharacter/Blueprints/Characters/BaseCharacter_BP.BaseCharacter_BP_C|GetCharacterTag _pawn_ai)) "NewEnumerator0")
      ;[1 1 1] Set the remaining recognize time to max recognize time
      (AI|Components|Blackboard|SetValueasFloat (AI|GetBlackboard 0) (Utilities|Name|MakeLiteralName "RemainRecognizeTime") (Utilities|Struct|BreakAI_Recognize_Struct (Utilities|Struct|BreakAI_Configs_Struct (Variables|/Game/UltimateCharacter/Blueprints/Characters/AICharacter_BP.AICharacter_BP_C|GetAIConfig _pawn_ai))))
      (Default|UpdateRecognitionBar (Variables|Internal|GetPawn_AI) 0.0)
      ;[1 1 1] AI don't need target after reset checkpoint
      (SetInfo|SetTarget))))