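; Base HUD for the player, creating and owning the main gameplay widget plus pause and game-over menus.
; InitializeUI builds the main widget from the pawn's attack types, then wrapper functions forward health, ammo, icons, score, combo, crosshair and messages to it.
; Menu toggles switch input mode and usually the cursor, with console commands pausing the game or slowing it while the inventory is open.
; Gamepad functions drive pause-menu and inventory navigation.
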(fn ConstructionScript)

(fn InitializeUI
  (params (InPawn :type Player%20Character%20BP%20Object%20Reference))
  (bind _playerowner (Variables|Default|GetPlayerOwner))
  (Debug|DebugMessage "BaseHUD_BP" "InitializeUI" "" "NewEnumerator0")
  ;[1 1 1] Create main widget and initialize by character attack types
  (Input|SetInputModeGameOnly _playerowner false)
  (bind _returnvalue (UserInterface|CreateWidget "/Game/UltimateCharacter/Blueprints/UMG/Base_WidgetBP.Base_WidgetBP_C" _playerowner))
  (bind _output_get (Variables|Internal|SetMainUI _returnvalue))
  (UserInterface|Viewport|AddtoViewport _output_get 0)
  (Default|InitializeAttackMenu (Variables|Internal|GetMainUI) (.Types (Utilities|Struct|BreakPlayer_Attacks_Struct (Variables|/Game/UltimateCharacter/Blueprints/Characters/PlayerCharacter_BP.PlayerCharacter_BP_C|GetPlayerAttacks InPawn))))
  (Widget|SetVisibility (Variables|/Game/UltimateCharacter/Blueprints/UMG/Base_WidgetBP.Base_WidgetBP_C|GetInventoryLayer (Variables|Internal|GetMainUI)) "Hidden")
  (UI|ToggleCrosshair)
  (Utilities|FlowControl|Sequence
    (:then_0
      (Utilities|IsValid (Variables|Internal|GetPauseUI)
        (:Is%20Valid
          (Widget|RemovefromParent (Variables|Internal|GetPauseUI)))
        (:Is%20Not%20Valid
          _))
      (Variables|Internal|SetPauseUI 0))
    (:then_1
      (Utilities|IsValid (Variables|Internal|GetGameOverUI)
        (:Is%20Valid
          (Widget|RemovefromParent (Variables|Internal|GetGameOverUI)))
        (:Is%20Not%20Valid
          _))
      (Variables|Internal|SetGameOverUI 0))))

(fn DebugMessage
  (params (InCallerName :type String) (InFunction :type String) (InMessage :type String) (InMessageType :type MessageType%20Enum :default "NewEnumerator0"))
  (if (or (Variables|Debug|GetbShowDebugMessage) (Utilities|Enum|Equal(Enum) InMessageType "NewEnumerator3"))
    (CallFunction|ShowDebugMessage InCallerName InFunction InMessage InMessageType)))

(fn ToggleInventory
  (params (bInAuto :type Boolean))
  (bind _mainui (Variables|Internal|GetMainUI))
  (bind _mainui_2 (Variables|Internal|GetMainUI))
  (bind _playerowner (Variables|Default|GetPlayerOwner))
  (bind _playerowner_2 (Variables|Default|GetPlayerOwner))
  (bind _inventorylayer (Variables|/Game/UltimateCharacter/Blueprints/UMG/Base_WidgetBP.Base_WidgetBP_C|GetInventoryLayer _mainui_2))
  (bind _crosshair_wbp (Variables|/Game/UltimateCharacter/Blueprints/UMG/Base_WidgetBP.Base_WidgetBP_C|GetCrosshair_WBP _mainui))
  (bind _crosshair (Variables|/Game/UltimateCharacter/Blueprints/UMG/Crosshair/Crosshair_WBP.Crosshair_WBP_C|GetCrosshair _crosshair_wbp))
  (bind _brush (Variables|/Script/UMG.Image|GetBrush _crosshair))
  (bind _resourceobject (Utilities|Struct|BreakSlateBrush _brush))
  (Debug|DebugMessage "BaseHUD_BP" "ToggleInventory" "" "NewEnumerator0")
  (if bInAuto
    ;[1 1 1] Toggle main menu & mouse cursor visibility, also if crosshair is set
    (Initialize|RefreshUI :!label _label)
    (Widget|SetVisibility _inventorylayer "Hidden")
    (Utilities|IsValid _resourceobject
      (:Is%20Valid
        (Widget|SetVisibility _crosshair_wbp "HitTestInvisible"))
      (:Is%20Not%20Valid
        _))
    (Variables|/Script/Engine.PlayerController|SetbShowMouseCursor _playerowner false)
    (Input|SetInputModeGameOnly _playerowner_2 false)
    (LocalVariables|SetTempVisibility "Hidden")
    (else
      (switch Utilities|FlowControl|Switch|SwitchonESlateVisibility (Widget|GetVisibility (Variables|/Game/UltimateCharacter/Blueprints/UMG/Base_WidgetBP.Base_WidgetBP_C|GetInventoryLayer (Variables|Internal|GetMainUI)))
        (:Visible
          (goto _label))
        (:Hidden
          (Audio|PlaySound2D "/Game/UltimateCharacter/Sounds/UI/Menu_OpeningSound.Menu_OpeningSound" 1.0 1.0 0.0 0 0)
          (Widget|SetVisibility _inventorylayer "Visible")
          (Utilities|IsValid _resourceobject
            (:Is%20Valid
              (Widget|SetVisibility _crosshair_wbp "Hidden"))
            (:Is%20Not%20Valid
              _))
          (Variables|/Script/Engine.PlayerController|SetbShowMouseCursor _playerowner true)
          (Input|SetInputModeGameandUI _playerowner_2 (Variables|Internal|GetMainUI) "LockAlways" true false)
          (LocalVariables|SetTempVisibility "Visible")))))
  ;[1 1 1] Slomo the game after open/close the menu
  (Development|ExecuteConsoleCommand (Utilities|Select :Index (LocalVariables|GetTempVisibility) :Visible "Slomo 0.1" :Collapsed "" :Hidden "Slomo 1" :HitTestInvisible "" :SelfHitTestInvisible "") (Variables|Default|GetPlayerOwner))
  (Variables|/Game/UltimateCharacter/Blueprints/UMG/Base_WidgetBP.Base_WidgetBP_C|SetGamepadTarget (Variables|Internal|GetMainUI) 0)
  (return (LocalVariables|GetTempVisibility)))

(fn RefreshUI
  (Debug|DebugMessage "BaseHUD_BP" "RefreshUI" "" "NewEnumerator0")
  (Utilities|IsValid (Variables|Internal|GetMainUI)
    (:Is%20Valid
      (Default|Refresh (Variables|Internal|GetMainUI)))
    (:Is%20Not%20Valid
      (Debug|DebugMessage "BaseHUD_BP" "RefreshUI" "MainUI is not valid" "NewEnumerator2"))))

(fn ToggleCrosshair
  (params (InTexture :type Texture%20Object%20Reference))
  (bind _mainui (Variables|Internal|GetMainUI))
  (bind _mainui_2 (Variables|Internal|GetMainUI))
  (bind _crosshair_wbp (Variables|/Game/UltimateCharacter/Blueprints/UMG/Base_WidgetBP.Base_WidgetBP_C|GetCrosshair_WBP _mainui))
  (bind _crosshair_wbp_2 (Variables|/Game/UltimateCharacter/Blueprints/UMG/Base_WidgetBP.Base_WidgetBP_C|GetCrosshair_WBP _mainui_2))
  (Debug|DebugMessage "BaseHUD_BP" "ToggleCrosshair" "" "NewEnumerator0")
  ;[1 1 1] Hide/Unhide crosshair, base on crosshair image
  (Default|ChangeCrosshair _crosshair_wbp_2 InTexture)
  (Utilities|IsValid (.ResourceObject (Utilities|Struct|BreakSlateBrush (Variables|/Script/UMG.Image|GetBrush (Variables|/Game/UltimateCharacter/Blueprints/UMG/Crosshair/Crosshair_WBP.Crosshair_WBP_C|GetCrosshair _crosshair_wbp_2))))
    (:Is%20Valid
      (Widget|SetVisibility _crosshair_wbp "Visible")
      (return "Visible"))
    (:Is%20Not%20Valid
      (Widget|SetVisibility _crosshair_wbp "Hidden")
      (return "Hidden"))))

(fn MessageReceived
  (params (InMessage :type Text) (InType :type MessageType%20Enum :default "NewEnumerator0"))
  (bind _mainui (Variables|Internal|GetMainUI))
  (Utilities|IsValid _mainui
    (:Is%20Valid
      ;[1 1 1] Add message to box
      (Default|AddMessage (Variables|/Game/UltimateCharacter/Blueprints/UMG/Base_WidgetBP.Base_WidgetBP_C|GetMessageBox_WBP _mainui) InMessage InType))
    (:Is%20Not%20Valid
      (Debug|DebugMessage "BaseHUD_BP" "MessageReceived" "Main UI is not valid" "NewEnumerator2"))))

(fn UpdateHealth
  (params (InPercent :type Float%20%28double-precision%29))
  ;[1 1 1] Update health bar
  (Default|UpdateHealth (Variables|/Game/UltimateCharacter/Blueprints/UMG/Base_WidgetBP.Base_WidgetBP_C|GetHealth_WBP (Variables|Internal|GetMainUI)) InPercent))

(fn ToggleBlockUMG
  (params (InEnable :type Boolean))
  ;[1 1 1] Toggle block button umg from main widget
  (Default|ToggleBlockUMG (Variables|Internal|GetMainUI) InEnable))

(fn UnequipItemIcon
  (params (InTag :type Name))
  ;[1 1 1] Remove icons from equipped list
  (Default|RemovefromIcons (Variables|Internal|GetMainUI) InTag))

(fn ToggleComboUI
  (params (InEnable :type Boolean) (InTexture :type Texture%20Object%20Reference))
  ;[1 1 1] Toggle combo icon on HUD
  (Default|ToggleComboUMG (Variables|Internal|GetMainUI) InEnable InTexture))

(fn EquipItemIcon
  (params (InTag :type Name) (Icon :type Texture%20Object%20Reference))
  ;[1 1 1] Remove icons from equipped list
  (Default|AddtoIcons (Variables|Internal|GetMainUI) InTag Icon))

(fn UpdateAmmo
  (params (InTag :type Name) (InClipAmmo :type Integer) (InClips :type Integer))
  (Default|UpdateAmmo (Variables|Internal|GetMainUI) InTag InClipAmmo InClips))

(fn DeathUI
  (Widget|RemovefromParent (Variables|Internal|GetMainUI)))

(fn PauseMenu
  (bind _mainui (Variables|Internal|GetMainUI))
  (Development|ExecuteConsoleCommand "pause" (Variables|Default|GetPlayerOwner))
  (Utilities|IsValid (Variables|Internal|GetPauseUI)
    (:Is%20Valid
      (Widget|RemovefromParent (Variables|Internal|GetPauseUI))
      (Variables|Internal|SetPauseUI 0)
      ;[1 1 1] Set focus to inventory
      (Utilities|IsValid _mainui
        (:Is%20Valid
          (if (Utilities|Enum|Equal(Enum) (Widget|GetVisibility (Variables|/Game/UltimateCharacter/Blueprints/UMG/Base_WidgetBP.Base_WidgetBP_C|GetInventoryLayer _mainui)) "Visible")
            (Input|SetInputModeGameandUI (Variables|Default|GetPlayerOwner) (Variables|/Game/UltimateCharacter/Blueprints/UMG/Base_WidgetBP.Base_WidgetBP_C|GetInventoryLayer (Variables|Internal|GetMainUI)) "DoNotLock" true false)
            (else
              (Input|SetInputModeGameOnly (Variables|Default|GetPlayerOwner) false :!label _label)
              (Variables|/Script/Engine.PlayerController|SetbShowMouseCursor (Variables|Default|GetPlayerOwner) false))))
        (:Is%20Not%20Valid
          (goto _label))))
    (:Is%20Not%20Valid
      ;[1 1 1] Set input mode to pause menu
      (bind _returnvalue (UserInterface|CreateWidget "/Game/UltimateCharacter/Blueprints/UMG/PauseMenu_WidgetBP.PauseMenu_WidgetBP_C" (Variables|Default|GetPlayerOwner)))
      (bind _output_get (Variables|Internal|SetPauseUI _returnvalue))
      (UserInterface|Viewport|AddtoViewport _output_get 0)
      (Input|SetInputModeGameandUI (Variables|Default|GetPlayerOwner) 0 "DoNotLock" false false)
      (Variables|/Script/Engine.PlayerController|SetbShowMouseCursor (Variables|Default|GetPlayerOwner) true))))

(fn MoveonPauseMenu
  (params (bInUp :type Boolean))
  (bind _pauseui (Variables|Internal|GetPauseUI))
  (bind _activebuttonindex (Variables|/Game/UltimateCharacter/Blueprints/UMG/PauseMenu_WidgetBP.PauseMenu_WidgetBP_C|GetActiveButtonIndex _pauseui))
  (Utilities|IsValid _pauseui
    (:Is%20Valid
      (bind _output_get (LocalVariables|SetTempIndex (Math|Integer|Clamp(Integer) (Math|Integer|SelectInt (- _activebuttonindex 1) (+ _activebuttonindex 1) bInUp) 0 (Utilities|Array|Length (Variables|/Game/UltimateCharacter/Blueprints/UMG/PauseMenu_WidgetBP.PauseMenu_WidgetBP_C|GetButtons _pauseui)))))
      (Default|ToggleActiveButton (Variables|Internal|GetPauseUI) _output_get))))

(fn SelectonPauseMenu
  (bind _pauseui (Variables|Internal|GetPauseUI))
  (Utilities|IsValid _pauseui
    (:Is%20Valid
      (Default|SelectMenu _pauseui))))

(fn RotateInventory
  (params (InDegree :type Float%20%28double-precision%29))
  (if (Internal|CheckInvetoryforGamepad)
    (Default|OnGamepadRotate (Variables|Internal|GetMainUI) (Math|Float|Truncate InDegree))))

(fn GampadSelectInventory
  (if (Internal|CheckInvetoryforGamepad)
    (Default|OnGamepadSelect (Variables|Internal|GetMainUI))))

(fn CheckInvetoryforGamepad
  (bind _mainui (Variables|Internal|GetMainUI))
  (Utilities|IsValid _mainui
    (:Is%20Valid
      (return (and (Utilities|Enum|Equal(Enum) (Widget|GetVisibility (Variables|/Game/UltimateCharacter/Blueprints/UMG/Base_WidgetBP.Base_WidgetBP_C|GetInventoryLayer _mainui)) "Visible") (not (Variables|/Game/UltimateCharacter/Blueprints/UMG/Base_WidgetBP.Base_WidgetBP_C|GetbMouseHover _mainui)))))
    (:Is%20Not%20Valid
      (return false))))

(fn GamepadBackMenu
  (if (Internal|CheckInvetoryforGamepad)
    (Default|OnGamepadBack (Variables|Internal|GetMainUI))))

(fn ToggleGameOver
  (Utilities|IsValid (Variables|Internal|GetGameOverUI)
    (:Is%20Valid
      (Widget|RemovefromParent (Variables|Internal|GetGameOverUI))
      (bind _asplayer_character_bp (Utilities|Casting|CastToPlayerCharacter_BP (Class|HUD|GetOwningPawn)))
      (Initialize|InitializeUI _asplayer_character_bp))
    (:Is%20Not%20Valid
      (Widget|RemovefromParent (Variables|Internal|GetMainUI))
      (bind _returnvalue (UserInterface|CreateWidget "/Game/UltimateCharacter/Blueprints/UMG/GameOverMenu_WidgetBP.GameOverMenu_WidgetBP_C" (Variables|Default|GetPlayerOwner)))
      (bind _output_get (Variables|Internal|SetGameOverUI _returnvalue))
      (Input|SetInputModeUIOnly (Variables|Default|GetPlayerOwner) _output_get "DoNotLock" false)
      (UserInterface|Viewport|AddtoViewport (Variables|Internal|GetGameOverUI) 0))))

(fn UpdateScore
  (params (InScore :type Integer) (InCombo :type Integer))
  (Utilities|IsValid (Variables|Internal|GetMainUI)
    (:Is%20Valid
      (Default|UpdateScore (Variables|/Game/UltimateCharacter/Blueprints/UMG/Base_WidgetBP.Base_WidgetBP_C|GetPlayerScore_WBP (Variables|Internal|GetMainUI)) InScore)
      (Default|UpdateCombo (Variables|/Game/UltimateCharacter/Blueprints/UMG/Base_WidgetBP.Base_WidgetBP_C|GetComboScore_WBP (Variables|Internal|GetMainUI)) InCombo))))

(fn SpawnScore
  (params (InScore :type Integer) (InLocation :type Vector))
  (bind _mainui (Variables|Internal|GetMainUI))
  (Utilities|IsValid _mainui
    (:Is%20Valid
      (Default|SpawnScore _mainui InScore InLocation))))

(fn ResetHUD
  (Utilities|FlowControl|Sequence
    (:then_0
      (Utilities|IsValid (Variables|Internal|GetMainUI)
        (:Is%20Valid
          (Widget|RemovefromParent (Variables|Internal|GetMainUI))
          (Variables|Internal|SetMainUI 0))))
    (:then_1
      (Utilities|IsValid (Variables|Internal|GetPauseUI)
        (:Is%20Valid
          (Widget|RemovefromParent (Variables|Internal|GetPauseUI))
          (Variables|Internal|SetPauseUI 0))))
    (:then_2
      (Utilities|IsValid (Variables|Internal|GetGameOverUI)
        (:Is%20Valid
          (Widget|RemovefromParent (Variables|Internal|GetGameOverUI))
          (Variables|Internal|SetGameOverUI 0))))))

(fn HideComboCounter
  (Widget|SetVisibility (Variables|/Game/UltimateCharacter/Blueprints/UMG/Base_WidgetBP.Base_WidgetBP_C|GetComboScore_WBP (Variables|Internal|GetMainUI)) "Hidden"))

(fn ShowFocusText
  (params (bInShow :type Boolean))
  (bind _mainui (Variables|Internal|GetMainUI))
  (Utilities|IsValid _mainui
    (:Is%20Valid
      (Widget|SetVisibility (Variables|/Game/UltimateCharacter/Blueprints/UMG/Base_WidgetBP.Base_WidgetBP_C|GetFocus_TXT _mainui) (select bInShow "HitTestInvisible" "Hidden")))))