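; BP_CheckPoint is a checkpoint actor that respawns the player and stored characters when reset.
; Its trigger activates it on first overlap, by any actor, and sets it as the player controller's current checkpoint if a player caused it.
; On reset, an active checkpoint respawns characters from stored class and transform data, calls CheckpointReset, then spawns and possesses a new player pawn at SpawnPoint and refreshes the HUD.
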(event OnComponentBeginOverlap(Trigger)
  (params (OverlappedComponent :type Primitive%20Component%20Object%20Reference) (OtherActor :type Actor%20Object%20Reference) (OtherComp :type Primitive%20Component%20Object%20Reference) (OtherBodyIndex :type Integer) (bFromSweep :type Boolean) (SweepResult :type Hit%20Result%20Structure%20%28by%20ref%29))
  ;[1 1 1] Trigger overlap
  (CallFunction|TriggerOverlap OtherActor))

(event EventBeginPlay)

(event Collision|EventActorBeginOverlap
  (params (OtherActor :type Actor%20Object%20Reference)))

(event EventTick
  (params (DeltaSeconds :type Float%20%28single-precision%29)))

(fn ConstructionScript)

(fn StoreCharacterData
  (params (InData :type F%20Checkpoint%20Data%20Structure))
  (Utilities|Array|Add (Variables|Internal|GetCheckpointData) InData)
  (Debug|DebugMessage "BP_Checkpoint" "ResetPlayer" "StoreCharacterData" "NewEnumerator0"))

(fn SpawnCharacters
  (Debug|DebugMessage "BP_Checkpoint" "SpawnCharacters" "" "NewEnumerator0")
  ;[1 1 1] Spawn all killed characters relevant to this check point
  (for _array_element (Variables|Internal|GetCheckpointData)
    (if (Utilities|IsValidClass (.SpawnClass (Utilities|Struct|BreakFCheckpointData _array_element)))
      (bind _returnvalue (Game|SpawnActorfromClass (.SpawnClass (Utilities|Struct|BreakFCheckpointData _array_element)) (Math|Transform|MakeTransform (.SpawnLocation (Utilities|Struct|BreakFCheckpointData _array_element)) (.SpawnRotation (Utilities|Struct|BreakFCheckpointData _array_element))) "AdjustIfPossibleButAlwaysSpawn" "SelectDefaultAtRuntime" 0 self 0))
      (Utilities|IsValid (Pawn|GetController _returnvalue)
        (:Is%20Not%20Valid
          (Pawn|SpawnDefaultController _returnvalue))))))

(fn ResetCharacters
  (Default|CallCheckpointReset)
  (Debug|DebugMessage "BP_Checkpoint" "ResetCharacters" "" "NewEnumerator0"))

(fn ResetCheckpoint
  (params (InPlayer :type Base%20Player%20Controller%20BP%20Object%20Reference))
  (if (Variables|Internal|GetbIsActive)
    (Debug|DebugMessage "BP_Checkpoint" "ResetCheckpoint" "" "NewEnumerator0")
    (Character|SpawnCharacters)
    (Character|ResetCharacters)
    (Character|ResetPlayer InPlayer)
    (else
      (Debug|DebugMessage "BP_Checkpoint" "ResetCheckpoint" "Checkpoint is not active" "NewEnumerator1"))))

(fn ResetPlayer
  (params (InPC :type Base%20Player%20Controller%20BP%20Object%20Reference))
  (bind _characterclass (Variables|/Game/UltimateCharacter/Blueprints/Characters/BasePlayerController_BP.BasePlayerController_BP_C|GetCharacterClass InPC))
  (bind _spawnpoint (Variables|Default|GetSpawnPoint))
  (Debug|DebugMessage "BP_Checkpoint" "ResetPlayer" "" "NewEnumerator0")
  (if (!= _characterclass 0)
    (bind _asbase_hud_bp (Utilities|Casting|CastToBaseHUD_BP (HUD|GetHUD InPC))
      (:then
        (Default|ResetHUD _asbase_hud_bp))
      (:CastFailed
        (Debug|DebugMessage "BP_Checkpoint" "ResetPlayer" "Cast to BaseHUD_BP failed!" "NewEnumerator2")))
    (bind _returnvalue (Game|SpawnActorfromClass _characterclass (Math|Transform|MakeTransform (Transformation|GetWorldLocation _spawnpoint) (Transformation|GetWorldRotation _spawnpoint)) "AdjustIfPossibleButAlwaysSpawn" "SelectDefaultAtRuntime" 0 0))
    (Pawn|Possess InPC _returnvalue)
    (bind _asbase_hud_bp_2 (Utilities|Casting|CastToBaseHUD_BP (HUD|GetHUD InPC)))
    (Default|UpdateScore _asbase_hud_bp_2 (Variables|/Game/UltimateCharacter/Blueprints/Characters/BasePlayerController_BP.BasePlayerController_BP_C|GetScore InPC))
    (else
      (Debug|DebugMessage "BP_Checkpoint" "ResetPlayer" "Player character ckass is not valid!" "NewEnumerator3"))))

(fn DebugMessage
  (params (InCallerName :type String) (InFunction :type String) (InMessage :type String) (InMessageType :type MessageType%20Enum :default "NewEnumerator0"))
  (if (or (Variables|Debug|GetbShowDebugMessage) (Utilities|Enum|Equal(Enum) InMessageType "NewEnumerator3"))
    (CallFunction|ShowDebugMessage InCallerName InFunction InMessage InMessageType)))

(fn TriggerOverlap
  (params (InActor :type Actor%20Object%20Reference))
  (Debug|DebugMessage "BP_Checkpoint" "TriggerOverlap" "" "NewEnumerator0")
  ;[1 1 1] Overlap trigger and if checkpoint is not active makes it active and set as current checkpoint in the player controller
  (if (Variables|Internal|GetbIsActive)
    (return false)
    (else
      (Variables|Internal|SetbIsActive true)
      (bind _asplayer_character_bp (Utilities|Casting|CastToPlayerCharacter_BP InActor)
        (:then
          (bind _asbase_player_controller_bp (Utilities|Casting|CastToBasePlayerController_BP (Pawn|GetController _asplayer_character_bp))
            (:then
              (Variables|/Game/UltimateCharacter/Blueprints/Characters/BasePlayerController_BP.BasePlayerController_BP_C|SetCurrentCheckpoint _asbase_player_controller_bp self)
              (return true))
            (:CastFailed
              (return false))))
        (:CastFailed
          (return false))))))