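; Blueprint function library of stateless helpers shared by UltimateCharacter player and AI characters.
; Combat helpers scale damage by health threshold and amounts by GameMode difficulty, and report alert and focus state; IsFriendlyDamage is a stub returning false.
; Movement and animation helpers compute facing angles, yaw-only interpolated rotation, gait values, montage playback and ground checks via downward line traces.
; Utilities provide cumulative-chance index selection, color-coded debug printing and FPS-scaled delta time.
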(fn CalculateHealthMultiplierDamage
  (params (InDamage :type Float%20%28double-precision%29) (InHealth :type Float%20%28double-precision%29) (InHealthMultiplier :type Health%20Multiplier%20Struct%20Structure))
  ;[1 1 1] Set local variables and check if the current health & damage are greater than zero
  (LocalVariables|SetTempHM InHealthMultiplier)
  (LocalVariables|SetTempHealth InHealth)
  (bind _output_get (LocalVariables|SetTempDamage InDamage))
  (if (and (> _output_get 0.0) (> (LocalVariables|GetTempHealth) 0.0))
    ;[1 1 1] If multiplier is zero so just return the actual damage
    (if (!= (.multiplier (LocalVariables|GetTempHM)) 0.0)
      ;[1 1 1] If threshold is not greater than 5 or is not less than current health then just return the actual damage
      (if (and (>= (.healththreshold (LocalVariables|GetTempHM)) 5.0) (<= (LocalVariables|GetTempHealth) (.healththreshold (LocalVariables|GetTempHM))))
        (return (+ (* (/ (* (Math|Float|Absolute(Float) (* (- 1e+02 (* (Math|Float|MapRangeClamped (LocalVariables|GetTempHealth) 0.0 (.healththreshold (LocalVariables|GetTempHM)) 0.0 1.0) 1e+02)) (.multiplier (LocalVariables|GetTempHM)))) (LocalVariables|GetTempDamage)) 1e+02) (Math|Float|SelectFloat 1.0 -1.0 (> (.multiplier (LocalVariables|GetTempHM)) 0.0))) (LocalVariables|GetTempDamage)))
        (else
          (return (LocalVariables|GetTempDamage))))
      (else
        (return (LocalVariables|GetTempDamage))))
    (else
      (return (LocalVariables|GetTempDamage)))))

(fn CalculateDifficultyMultiplier
  (params (InAmount :type Float%20%28double-precision%29) (InDifficultyInfo :type Difficulty%20Multiplier%20Struct%20Structure) (InCurrentDifficulty :type Difficulty_Enum%20Enum :default "NewEnumerator0"))
  (bind (_easy _normal _hard) (Utilities|Struct|BreakDifficultyMultiplier_Struct InDifficultyInfo))
  ;[1 1 1] Calculate multiplier to input amount by game difficulty
  (switch Utilities|FlowControl|Switch|SwitchonDifficulty_Enum InCurrentDifficulty
    (:NewEnumerator0
      (return (* InAmount (select (> _easy 0.0) _easy 1.0))))
    (:NewEnumerator1
      (return (* InAmount (select (> _normal 0.0) _normal 1.0))))
    (:NewEnumerator2
      (return (* InAmount (select (> _hard 0.0) _hard 1.0))))))

(fn AngleDifference
  (params (InActorRotation :type Rotator) (InActorLocation :type Vector) (InTargetLocation :type Vector))
  (bind (_x _y) (Math|Vector|BreakVector InActorLocation))
  (bind (_x_2 _y_2) (Math|Vector|BreakVector InTargetLocation))
  (return (Class|KismetMathLibrary|DegAcos (Math|Vector|DotProduct (Math|Vector|Normalize (Math|Vector|GetForwardVector InActorRotation)) (Math|Vector|Normalize (- (Math|Vector|MakeVector _x_2 _y_2 0.0) (Math|Vector|MakeVector _x _y 0.0)))))))

(fn RotatetoTarget
  (params (InActor :type Actor%20Object%20Reference) (InTarget :type Actor%20Object%20Reference) (Speed :type Float%20%28double-precision%29))
  (return (Math|Interpolation|RInterpTo (Transformation|GetActorRotation InActor) (Math|Rotator|MakeRotator 0.0 0.0 (.yaw (Math|Rotator|FindLookatRotation (Transformation|GetActorLocation InActor) (Transformation|GetActorLocation InTarget)))) (Utilities|Time|GetWorldDeltaSeconds) Speed)))

(fn GetGameDifficulty
  (bind _asgame_mode_bp (Utilities|Casting|CastToGameMode_BP (Game|GetGameMode))
    (:then
      (return (Default|GetDifficulty _asgame_mode_bp)))
    (:CastFailed
      (return "NewEnumerator1"))))

(fn IsFriendlyDamage
  (params (InDamageCauser :type Base%20Character%20BP%20Object%20Reference) (InDamageTaker :type Base%20Character%20BP%20Object%20Reference))
  (return false))

(fn IsPlayingAnimMontage
  (params (InSkeletalMesh :type Skeletal%20Mesh%20Component%20Object%20Reference))
  (return (Class|AnimInstance|IsAnyMontagePlaying (Components|SkeletalMesh|GetAnimInstance InSkeletalMesh))))

(fn SelectIndexUsingChance
  (params (InArrayChances :type Array%20of%20Integers))
  (if (> (Utilities|Array|Length InArrayChances) 0)
    (LocalVariables|SetTempRand (Math|Random|RandomIntegerinRange 0 99))
    (bind (_array_element _array_index) (Utilities|Array|ForEachLoopwithBreak InArrayChances :!label _label)
      (:LoopBody
        (bind _output_get (LocalVariables|SetCurrentRange (+ _array_element (LocalVariables|GetCurrentRange))))
        (if (< (LocalVariables|GetTempRand) _output_get)
          (LocalVariables|SetDesiredIndex _array_index)
          (goto _label Break)))
      (:Completed
        (return (LocalVariables|GetDesiredIndex))))
    (else
      (return (LocalVariables|GetDesiredIndex)))))

(fn ShowDebugMessage
  (params (InCallerName :type String) (InFunction :type String) (InMessage :type String) (InMessageType :type MessageType%20Enum :default "NewEnumerator0"))
  (switch Utilities|FlowControl|Switch|SwitchonMessageType InMessageType
    (:NewEnumerator0
      _)
    (:NewEnumerator1
      _)
    (:NewEnumerator2
      _)
    (:NewEnumerator3
      _))
  (Development|PrintString 0 (Utilities|String|Append (Utilities|String|EnumtoString InMessageType) "-" InCallerName " - " InFunction " : " InMessage) true true (Utilities|Select :Index InMessageType :NewEnumerator0 "(R=0.000000,G=1.000000,B=0.000000,A=1.000000)" :NewEnumerator1 "(R=1.000000,G=1.000000,B=0.000000,A=1.000000)" :NewEnumerator2 "(R=1.000000,G=0.000000,B=0.000000,A=1.000000)" :NewEnumerator3 "(R=1.000000,G=0.000000,B=0.000000,A=1.000000)")))

(fn IsinAlert
  (params (InCharacater :type Base%20Character%20BP%20Object%20Reference))
  ;[1 1 1] Check AI alert state otherwise check the equipped weapons count
  (Utilities|IsValid InCharacater
    (:Is%20Valid
      (bind _asaicharacter_bp (Utilities|Casting|CastToAICharacter_BP InCharacater)
        (:then
          (return (Variables|/Game/UltimateCharacter/Blueprints/Characters/AICharacter_BP.AICharacter_BP_C|GetbInAlert _asaicharacter_bp)))
        (:CastFailed
          (return (> (Utilities|Array|Length (Variables|/Game/UltimateCharacter/Blueprints/Characters/BaseCharacter_BP.BaseCharacter_BP_C|GetEquippedWeapons InCharacater)) 0)))))
    (:Is%20Not%20Valid
      (return false))))

(fn ShowJumpAnimation
  (params (InCharacter :type Base%20Character%20BP%20Object%20Reference) (InHeight :type Float%20%28double-precision%29))
  (bind _returnvalue (Transformation|GetActorLocation InCharacter))
  (bind _capsulecomponent (Variables|/Script/Engine.Character|GetCapsuleComponent InCharacter))
  (bind (_x _y _z) (Math|Vector|BreakVector _returnvalue))
  (bind _capsulehalfheight (Variables|/Script/Engine.CapsuleComponent|GetCapsuleHalfHeight _capsulecomponent))
  (bind _returnvalue_2 (- _z _capsulehalfheight))
  (bind _returnvalue_3 (Math|Vector|MakeVector _x _y _returnvalue_2))
  (bind _returnvalue_4 (Collision|LineTraceByChannel 0 _returnvalue_3 (+ _returnvalue_3 (Math|Vector|MakeVector 0.0 0.0 (* (Math|Float|Absolute(Float) InHeight) -1.0))) "TraceTypeQuery1" false (Utilities|Array|MakeArray InCharacter) "None"))
  (return (not _returnvalue_4)))

(fn DistancetoGround
  (params (InCharacter :type Base%20Character%20BP%20Object%20Reference))
  (bind _returnvalue (Transformation|GetActorLocation InCharacter))
  (bind (_x _y _z) (Math|Vector|BreakVector _returnvalue))
  ;[1 1 1] Calculate distance to ground from bottom of capsule component
  (bind _output_get (LocalVariables|SetCharacterFoot (Math|Vector|MakeVector _x _y (- _z (Variables|/Script/Engine.CapsuleComponent|GetCapsuleHalfHeight (Variables|/Script/Engine.Character|GetCapsuleComponent InCharacter))))))
  (bind (_outhit _returnvalue_2) (Collision|LineTraceByChannel 0 _output_get (+ (LocalVariables|GetCharacterFoot) (* (Transformation|GetActorUpVector InCharacter) -1e+03)) "TraceTypeQuery1" false (Utilities|Array|MakeArray InCharacter) "None"))
  (if _returnvalue_2
    (return (Math|Vector|VectorLength (- (LocalVariables|GetCharacterFoot) (.Location (Collision|BreakHitResult _outhit)))))
    (else
      (return -1.0))))

(fn UpdateGaitSpeed
  (params (InSpeed :type Float%20%28double-precision%29) (InCharacter :type Base%20Character%20BP%20Object%20Reference))
  (bind _defaultmaxspeed (Variables|/Game/UltimateCharacter/Blueprints/Characters/BaseCharacter_BP.BaseCharacter_BP_C|GetDefaultMaxSpeed InCharacter))
  (bind _runningmodifier (Variables|/Game/UltimateCharacter/Blueprints/Characters/BaseCharacter_BP.BaseCharacter_BP_C|GetRunningModifier InCharacter))
  (bind _returnvalue (/ _defaultmaxspeed 2.0))
  (bind _returnvalue_2 (* _defaultmaxspeed _runningmodifier))
  (return (select (> InSpeed _returnvalue_2) (Math|Float|MapRangeClamped InSpeed _defaultmaxspeed _returnvalue_2 2.0 3.0) (select (> InSpeed _returnvalue) (Math|Float|MapRangeClamped InSpeed _returnvalue _defaultmaxspeed 1.0 2.0) (Math|Float|MapRangeClamped InSpeed 0.0 _returnvalue 0.0 1.0)))))

(fn GetModifiedDeltaTime
  (return (* (Math|Float|MapRangeClamped (/ 1.0 (Utilities|Time|GetWorldDeltaSeconds)) 3e+01 1.2e+02 0.25 1.0) (Utilities|Time|GetWorldDeltaSeconds))))

(fn IsinFocus
  (params (InPawn :type Base%20Character%20BP%20Object%20Reference))
  (bind _asplayer_character_bp (Utilities|Casting|CastToPlayerCharacter_BP InPawn)
    (:then
      (bind _boutfocus (Default|IsFocusonActor _asplayer_character_bp))
      (return _boutfocus))
    (:CastFailed
      (return false))))